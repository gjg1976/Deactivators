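; Wall border tile actor for the building system, placed at a given location with its current rotation and scale.
; Initialize stores the tile ID, assigns the border mesh and creates a dynamic material using the Ceiling concrete, offset by row and column.
; CreateMID also maps other wall types to marble, glass or concrete.
; The grid position from CalculateLocation goes unused, and OnInteract only reports whether the material instance is valid.
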(fn `CalculateLocation`
  (returns (OutLocation :type "Vector Structure"))
  (bind (_coordinate_row _coordinate_column) (break `/Game/Blueprints/Building/Tiles/S_Azi_Coordinate` (`self.Coordinate`)))
  (bind _x (.x (`.BoxExtent` (`KismetSystemLibrary.GetComponentBounds` null))))
  (bind _y (.y (`.BoxExtent` (`KismetSystemLibrary.GetComponentBounds` null))))
  (return (`KismetMathLibrary.MakeVector` (+ (* _x _coordinate_column 2.0) _x) (+ _y (* _y _coordinate_row 2.0)) (.z (`.BoxExtent` (`KismetSystemLibrary.GetComponentBounds` null))))))

(fn `CreateMID`
  (params (InWallID :type "/Game/Blueprints/Building/Wall/E_Dea_WallID Enum" :default "NewEnumerator0") (Random :type Integer))
  (bind (_coordinate_row _coordinate_column) (break `/Game/Blueprints/Building/Tiles/S_Azi_Coordinate` (`self.Coordinate`)))
  (bind _returnvalue (`PrimitiveComponent.CreateDynamicMaterialInstance` (`self.SM_wallborder`) 0 (select `/Game/Blueprints/Building/Wall/E_Dea_WallID` (`local.InWallID`) :`NewEnumerator0` "/Game/Materials/Tiles/MaterialsInstances/MI_TileConcrete6.MI_TileConcrete6" :`NewEnumerator1` (select `int` Random :`0` "/Game/Materials/Tiles/MaterialsInstances/MI_TileMarble1.MI_TileMarble1" :`1` "/Game/Materials/Tiles/MaterialsInstances/MI_TileMarble11.MI_TileMarble11" :`2` "/Game/Materials/Tiles/MaterialsInstances/MI_TileMarble14.MI_TileMarble14" :`3` "/Game/Materials/Tiles/MaterialsInstances/MI_TileMarble15.MI_TileMarble15" :`4` "/Game/Materials/Tiles/MaterialsInstances/MI_TileMarble16.MI_TileMarble16" :`5` "/Game/Materials/Tiles/MaterialsInstances/MI_TileMarble17.MI_TileMarble17" :`6` "/Game/Materials/Tiles/MaterialsInstances/MI_TileMarble18.MI_TileMarble18" :`7` "/Game/Materials/Tiles/MaterialsInstances/MI_TileMarble20.MI_TileMarble20" :`8` "/Game/Materials/Tiles/MaterialsInstances/MI_TileMarble33.MI_TileMarble33" :!type "MaterialInterface Object Reference") :`NewEnumerator2` "/Game/Materials/Tiles/Materials/M_Glass.M_Glass" :`NewEnumerator3` "/Game/Materials/Tiles/Materials/M_TileConcrete2.M_TileConcrete2" :`NewEnumerator4` "/Game/Materials/Tiles/Materials/M_TileConcrete2.M_TileConcrete2" :`NewEnumerator5` "/Game/Materials/Tiles/Materials/M_TileConcrete2.M_TileConcrete2") "None"))
  (bind _output_get (set `self.MID` _returnvalue))
  (`MaterialInstanceDynamic.SetScalarParameterValue` _output_get "Offset_X" (`KismetMathLibrary.Conv_IntToDouble` _coordinate_row))
  (`MaterialInstanceDynamic.SetScalarParameterValue` _output_get "Offset_Y" (`KismetMathLibrary.Conv_IntToDouble` _coordinate_column)))

(fn `GetBound`
  (returns (Bound :type "Vector Structure"))
  (return (`.BoxExtent` (`KismetSystemLibrary.GetComponentBounds` null))))

(fn `Initialize`
  (params (InTileID :type Integer) (InLocation :type "Vector Structure"))
  (bind (_returnvalue_location _returnvalue_rotation _returnvalue_scale) (`KismetMathLibrary.BreakTransform` (`self.GetTransform` (`ActorComponent.GetOwner` (`self.SM_wallborder`)))))
  (set `self.TileID` InTileID)
  (`self.SetMesh`)
  (`self.CalculateLocation`)
  (`self.K2_SetActorTransform` (`KismetMathLibrary.MakeTransform` InLocation _returnvalue_rotation _returnvalue_scale)))

(fn `OnInteract`
  (params (InColorMode :type "/Game/Blueprints/Building/Tiles/E_Azi_Colors Enum" :default "NewEnumerator0"))
  (returns (bSucess :type Boolean))
  (`self.MID`
    (:`then`
      (return true))
    (:`else`
      (return false))))

(fn `SetMesh`
  (`StaticMeshComponent.SetStaticMesh` (`self.SM_wallborder`) "/Game/Blueprints/Assets/Meshes/SM_wallborder.SM_wallborder")
  (`self.CreateMID` "NewEnumerator0"))

(fn `UserConstructionScript`)