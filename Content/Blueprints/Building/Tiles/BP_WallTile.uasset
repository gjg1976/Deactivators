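; BP_WallTile is a grid tile for building walls that can hold a decoration or an asset such as a teleporter or elevator.
; Initialize sets the mesh, positions the tile from its row/column and mesh bounds, and creates a ceiling dynamic material offset by coordinate.
; AddDecoration and AddAsset destroy attached actors, then spawn and attach the selected Blueprint.
; IsWalkable uses a box trace to report whether the tile is unobstructed.
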(event `self.ReceiveActorOnClicked`
  (params (ButtonPressed :type "Key Structure")))

(event `self.ReceiveBeginPlay`)

(fn `AddAsset`
  (bind _returnvalue (`KismetMathLibrary.MakeTransform` (`self.K2_GetActorLocation`) (`self.K2_GetActorRotation`)))
  (`self.ClearDecoration`)
  (switch `/Game/Blueprints/Building/Wall/E_Dea_WallAsset` (`self.Asset`)
    (:`NewEnumerator8`
      (bind _returnvalue_2 (`|SpawnActorFromClass` "/Game/Blueprints/Assets/BP_teleporter.BP_teleporter_C" _returnvalue "Undefined" "MultiplyWithRoot" self null))
      (if (> (`self.TileID`) 7)
        (`self.K2_AddActorLocalRotation` (struct :`Yaw` 180.0)))
      (`self.K2_AttachToActor` _returnvalue_2 self "None" "SnapToTarget" "SnapToTarget" "KeepRelative" false))
    (:`NewEnumerator9`
      (bind _returnvalue_3 (`|SpawnActorFromClass` "/Game/Blueprints/Assets/BP_elevator.BP_elevator_C" _returnvalue "Undefined" "MultiplyWithRoot" self null))
      (`self.K2_AttachToActor` _returnvalue_3 self "None" "SnapToTarget" "SnapToTarget" "KeepRelative" false))))

(fn `AddDecoration`
  (bind _returnvalue (`KismetMathLibrary.MakeTransform` (`self.K2_GetActorLocation`) (`self.K2_GetActorRotation`)))
  (`self.ClearDecoration`)
  (switch `/Game/Blueprints/Building/Wall/E_Dea_WallDecoration` (`self.Decoration`)
    (:`NewEnumerator1`
      (bind _returnvalue_2 (`|SpawnActorFromClass` "/Game/Blueprints/Decoration/BP_Clock.BP_Clock_C" _returnvalue "Undefined" "MultiplyWithRoot" self null))
      (`self.K2_AttachToActor` _returnvalue_2 self "None" "SnapToTarget" "SnapToTarget" "KeepRelative" false))
    (:`NewEnumerator2`
      (bind _returnvalue_3 (`|SpawnActorFromClass` "/Game/Blueprints/Decoration/BP_FireExtinghisher.BP_FireExtinghisher_C" _returnvalue "Undefined" "MultiplyWithRoot" self null))
      (`self.K2_AttachToActor` _returnvalue_3 self "None" "SnapToTarget" "SnapToTarget" "KeepRelative" false))
    (:`NewEnumerator4`
      (bind _returnvalue_4 (`|SpawnActorFromClass` "/Game/Blueprints/Decoration/BP_FireHydrant.BP_FireHydrant_C" _returnvalue "Undefined" "MultiplyWithRoot" self null))
      (`self.K2_AttachToActor` _returnvalue_4 self "None" "SnapToTarget" "SnapToTarget" "KeepRelative" false))
    (:`NewEnumerator5`
      (bind _returnvalue_5 (`|SpawnActorFromClass` "/Game/Blueprints/Decoration/BP_LedLamp.BP_LedLamp_C" _returnvalue "Undefined" "MultiplyWithRoot" self null))
      (`self.K2_AttachToActor` _returnvalue_5 self "None" "SnapToTarget" "SnapToTarget" "KeepRelative" false))
    (:`NewEnumerator6`
      (bind _returnvalue_6 (`|SpawnActorFromClass` "/Game/Blueprints/Decoration/BP_CeilingLight.BP_CeilingLight_C" _returnvalue "Undefined" "MultiplyWithRoot" self null))
      (`self.K2_AttachToActor` _returnvalue_6 self "None" "SnapToTarget" "SnapToTarget" "KeepRelative" false))
    (:`NewEnumerator7`
      (bind _returnvalue_7 (`|SpawnActorFromClass` "/Game/Blueprints/Decoration/BP_FrameYoungGirl.BP_FrameYoungGirl_C" _returnvalue "Undefined" "MultiplyWithRoot" self null))
      (`self.K2_AttachToActor` _returnvalue_7 self "None" "SnapToTarget" "SnapToTarget" "KeepRelative" false))
    (:`NewEnumerator8`
      (bind _returnvalue_8 (`|SpawnActorFromClass` "/Game/Blueprints/Decoration/BP_FramePopArt.BP_FramePopArt_C" _returnvalue "Undefined" "MultiplyWithRoot" self null))
      (`self.K2_AttachToActor` _returnvalue_8 self "None" "SnapToTarget" "SnapToTarget" "KeepRelative" false))
    (:`NewEnumerator9`
      (bind _returnvalue_9 (`|SpawnActorFromClass` "/Game/Blueprints/Decoration/BP_Pipe.BP_Pipe_C" _returnvalue "Undefined" "MultiplyWithRoot" self null))
      (`self.K2_AttachToActor` _returnvalue_9 self "None" "SnapToTarget" "SnapToTarget" "KeepRelative" false))
    (:`NewEnumerator10`
      (bind _returnvalue_10 (`|SpawnActorFromClass` "/Game/Blueprints/Decoration/BP_WallLamp.BP_WallLamp_C" _returnvalue "Undefined" "MultiplyWithRoot" self null))
      (`self.K2_AttachToActor` _returnvalue_10 self "None" "SnapToTarget" "SnapToTarget" "KeepRelative" false))
    (:`NewEnumerator11`
      (bind _returnvalue_11 (`|SpawnActorFromClass` "/Game/Blueprints/Decoration/BP_Alarm.BP_Alarm_C" _returnvalue "Undefined" "MultiplyWithRoot" self null))
      (`self.K2_AttachToActor` _returnvalue_11 self "None" "SnapToTarget" "SnapToTarget" "KeepRelative" false))
    (:`NewEnumerator12`
      (bind _returnvalue_12 (`|SpawnActorFromClass` "/Game/Blueprints/Decoration/BP_BattleActium.BP_BattleActium_C" _returnvalue "Undefined" "MultiplyWithRoot" self null))
      (`self.K2_AttachToActor` _returnvalue_12 self "None" "SnapToTarget" "SnapToTarget" "KeepRelative" false))
    (:`NewEnumerator13`
      (bind _returnvalue_13 (`|SpawnActorFromClass` "/Game/Blueprints/Decoration/BP_TigerHunt.BP_TigerHunt_C" _returnvalue "Undefined" "MultiplyWithRoot" self null))
      (`self.K2_AttachToActor` _returnvalue_13 self "None" "SnapToTarget" "SnapToTarget" "KeepRelative" false))
    (:`NewEnumerator14`
      (bind _returnvalue_14 (`|SpawnActorFromClass` "/Game/Blueprints/Decoration/BP_WallSconce.BP_WallSconce_C" _returnvalue "Undefined" "MultiplyWithRoot" self null))
      (`self.K2_AttachToActor` _returnvalue_14 self "None" "SnapToTarget" "SnapToTarget" "KeepRelative" false))
    (:`NewEnumerator15`
      (bind _returnvalue_15 (`|SpawnActorFromClass` "/Game/Blueprints/Decoration/BP_MetalGrid.BP_MetalGrid_C" _returnvalue "Undefined" "MultiplyWithRoot" self null))
      (`self.K2_AttachToActor` _returnvalue_15 self "None" "SnapToTarget" "SnapToTarget" "KeepRelative" false))))

(fn `CalculateLocation`
  (returns (OutLocation :type "Vector Structure"))
  (bind (_coordinate_row _coordinate_column) (break `/Game/Blueprints/Building/Tiles/S_Azi_Coordinate` (`self.Coordinate`)))
  (bind _x (.x (`.BoxExtent` (`KismetSystemLibrary.GetComponentBounds` (`self.SM_walltile`)))))
  (bind _y (.y (`.BoxExtent` (`KismetSystemLibrary.GetComponentBounds` (`self.SM_walltile`)))))
  (return (`KismetMathLibrary.MakeVector` (+ (* _x _coordinate_column 2.0) _x) (+ _y (* _y _coordinate_row 2.0)) (.z (`.BoxExtent` (`KismetSystemLibrary.GetComponentBounds` (`self.SM_walltile`)))))))

(fn `ClearDecoration`
  (bind (_arrayindex _arrayelement) (`/Engine/EditorBlueprintResources/StandardMacros.ReverseForEachLoop` (`self.GetAttachedActors` true))
    (:`LoopBody`
      (`self.K2_DestroyActor` _arrayelement))))

(fn `CreateMID`
  (params (InWallID :type "/Game/Blueprints/Building/Wall/E_Dea_WallID Enum" :default "NewEnumerator0") (Random :type Integer))
  (bind (_coordinate_row _coordinate_column) (break `/Game/Blueprints/Building/Tiles/S_Azi_Coordinate` (`self.Coordinate`)))
  (bind _returnvalue (`PrimitiveComponent.CreateDynamicMaterialInstance` (`self.SM_walltile`) 0 (select `/Game/Blueprints/Building/Wall/E_Dea_WallID` (`local.InWallID`) :`NewEnumerator0` "/Game/Materials/Tiles/MaterialsInstances/MI_TileConcrete6.MI_TileConcrete6" :`NewEnumerator1` (select `int` Random :`0` "/Game/Materials/Tiles/MaterialsInstances/MI_TileMarble1.MI_TileMarble1" :`1` "/Game/Materials/Tiles/MaterialsInstances/MI_TileMarble11.MI_TileMarble11" :`2` "/Game/Materials/Tiles/MaterialsInstances/MI_TileMarble14.MI_TileMarble14" :`3` "/Game/Materials/Tiles/MaterialsInstances/MI_TileMarble15.MI_TileMarble15" :`4` "/Game/Materials/Tiles/MaterialsInstances/MI_TileMarble16.MI_TileMarble16" :`5` "/Game/Materials/Tiles/MaterialsInstances/MI_TileMarble17.MI_TileMarble17" :`6` "/Game/Materials/Tiles/MaterialsInstances/MI_TileMarble18.MI_TileMarble18" :`7` "/Game/Materials/Tiles/MaterialsInstances/MI_TileMarble20.MI_TileMarble20" :`8` "/Game/Materials/Tiles/MaterialsInstances/MI_TileMarble33.MI_TileMarble33" :!type "MaterialInterface Object Reference") :`NewEnumerator2` "/Game/Materials/Tiles/Materials/M_Glass.M_Glass" :`NewEnumerator3` "/Game/Materials/Tiles/Materials/M_TileConcrete2.M_TileConcrete2" :`NewEnumerator4` "/Game/Materials/Tiles/Materials/M_TileConcrete2.M_TileConcrete2" :`NewEnumerator5` "/Game/Materials/Tiles/Materials/M_TileConcrete2.M_TileConcrete2") "None"))
  (bind _output_get (set `self.MID` _returnvalue))
  (`MaterialInstanceDynamic.SetScalarParameterValue` _output_get "Offset_X" (`KismetMathLibrary.Conv_IntToDouble` _coordinate_row))
  (`MaterialInstanceDynamic.SetScalarParameterValue` _output_get "Offset_Y" (`KismetMathLibrary.Conv_IntToDouble` _coordinate_column)))

(fn `GetBound`
  (returns (Bound :type "Vector Structure"))
  (return (`.BoxExtent` (`KismetSystemLibrary.GetComponentBounds` (`self.SM_walltile`)))))

(fn `GetTraceStartLocation`
  (returns (OutLocation :type "Vector Structure"))
  (return (+ (`self.K2_GetActorLocation`) (* (`self.GetActorUpVector`) 10.0))))

(fn `Initialize`
  (params (InTileID :type Integer))
  (bind (_returnvalue_location _returnvalue_rotation _returnvalue_scale) (`KismetMathLibrary.BreakTransform` (`self.GetTransform` (`ActorComponent.GetOwner` (`self.SM_walltile`)))))
  (set `self.TileID` InTileID)
  (`self.SetMesh`)
  (bind _outlocation (`self.CalculateLocation`))
  (`self.K2_SetActorTransform` (`KismetMathLibrary.MakeTransform` (+ _outlocation _returnvalue_location) _returnvalue_rotation _returnvalue_scale)))

(fn `IsWalkable`
  (returns (bOutWalkable :type Boolean))
  (return (not (`self.TraceOnBox`))))

(fn `OnInteract`
  (params (InColorMode :type "/Game/Blueprints/Building/Tiles/E_Azi_Colors Enum" :default "NewEnumerator0"))
  (returns (bSucess :type Boolean))
  (`self.MID`
    (:`then`
      (return true))
    (:`else`
      (return false))))

(fn `SetMesh`
  (`StaticMeshComponent.SetStaticMesh` (`self.SM_walltile`) "/Game/Blueprints/Assets/Meshes/SM_walltile.SM_walltile")
  (`self.CreateMID` "NewEnumerator0"))

(fn `TraceOnBox`
  (returns (bSuccess :type Boolean) (OutHit :type "HitResult Structure"))
  (bind (_outhit _returnvalue) (`KismetSystemLibrary.BoxTraceSingle` (`self.GetTraceStartLocation`) (`self.K2_GetActorLocation`) (* (+ (`.BoxExtent` (`KismetSystemLibrary.GetComponentBounds` null)) (* (`self.GetActorUpVector`) 5.0)) 0.9) (struct) "TraceTypeQuery1" false (`|MakeArray` self :!type "Actor Object Reference")))
  (return _returnvalue _outhit))

(fn `TraceOnHexagon`
  (params (bInPointTop :type Boolean))
  (returns (bSuccess :type Boolean) (OutHit :type "HitResult Structure"))
  (`KismetSystemLibrary.CapsuleTraceSingle` (`self.GetTraceStartLocation`) (`self.K2_GetActorLocation`) (* (`KismetMathLibrary.SelectFloat` (.x (`.BoxExtent` (`KismetSystemLibrary.GetComponentBounds` null))) (.y (`.BoxExtent` (`KismetSystemLibrary.GetComponentBounds` null))) (`local.bInPointTop`)) 0.9) 30.0 "TraceTypeQuery1")
  (return false))

(fn `UserConstructionScript`)