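; Grid tile actor for square or two hexagon layouts, serving as a pathfinding node with cost and parent data.
; Initialize sets the mesh, places the hidden tile from row/column and owner location, offsetting alternate hex lines.
; Walkability combines a force-block flag with shape traces, though the hexagon trace always reports no hit.
; A dynamic material shows interaction states and blocked or extra-cost shading; ExtraCost counts in both G and F.
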(event `self.ReceiveBeginPlay`
  (`self.CreateMID`))

(fn `CalculateLocation`
  (params (InType :type "/Game/Blueprints/EGridType Enum" :default "NewEnumerator0"))
  (returns (OutLocation :type "Vector Structure"))
  (bind _returnvalue (`self.GetOwner`))
  (bind (_coordinate_row _coordinate_column) (break `/Game/Blueprints/Building/Tiles/S_Azi_Coordinate` (`self.Coordinate`)))
  (bind _coordinate_row_2 (break `/Game/Blueprints/Building/Tiles/S_Azi_Coordinate` (`self.Coordinate`)))
  (bind (_coordinate_row_3 _coordinate_column_2) (break `/Game/Blueprints/Building/Tiles/S_Azi_Coordinate` (`self.Coordinate`)))
  (bind (_coordinate_row_4 _coordinate_column_3) (break `/Game/Blueprints/Building/Tiles/S_Azi_Coordinate` (`self.Coordinate`)))
  (bind (_coordinate_row_5 _coordinate_column_4) (break `/Game/Blueprints/Building/Tiles/S_Azi_Coordinate` (`self.Coordinate`)))
  (bind _x (.x (`.BoxExtent` (`KismetSystemLibrary.GetComponentBounds` (`self.Tile`)))))
  (bind _y (.y (`.BoxExtent` (`KismetSystemLibrary.GetComponentBounds` (`self.Tile`)))))
  (bind _z (.z (`.BoxExtent` (`KismetSystemLibrary.GetComponentBounds` (`self.Tile`)))))
  (bind _returnvalue_2 (* _x 2.0 _coordinate_column_4))
  (bind _returnvalue_3 (* _y 2.0 _coordinate_row))
  (bind _returnvalue_4 (select `/Game/Blueprints/EGridType` InType :`NewEnumerator0` (`KismetMathLibrary.MakeVector` (* _x _coordinate_column_2 2.0) (* _y _coordinate_row_3 2.0) _z) :`NewEnumerator1` (`KismetMathLibrary.MakeVector` (`KismetMathLibrary.SelectFloat` _returnvalue_2 (+ _returnvalue_2 _x) (== (mod _coordinate_row_5 2) 0)) (* _y 2.0 _coordinate_row_2 (/ 3.0 4.0)) _z) :`NewEnumerator2` (`KismetMathLibrary.MakeVector` (* _x 2.0 _coordinate_column_3 (/ 3.0 4.0)) (`KismetMathLibrary.SelectFloat` _returnvalue_3 (+ _returnvalue_3 _y) (== (mod _coordinate_column 2) 0)) _z)))
  (`/Engine/EditorBlueprintResources/StandardMacros.IsValid` _returnvalue
    (:`Is Valid`
      (return (+ (`self.K2_GetActorLocation` _returnvalue) _returnvalue_4)))
    (:`Is Not Valid`
      (return _returnvalue_4))))

(fn `CreateMID`
  (bind _returnvalue (`PrimitiveComponent.CreateDynamicMaterialInstance` (`self.Tile`) 0 "/Game/Materials/Tiles/Materials/M_Tile.M_Tile" "None"))
  (bind _output_get (set `self.MID` _returnvalue))
  (`MaterialInstanceDynamic.SetVectorParameterValue` _output_get "Color" (`self.NormalColor`)))

(fn `GetCost_F`
  (returns (Cost :type Integer))
  (bind (_parent _cost_g _cost_h) (break `/Game/Blueprints/Building/Tiles/S_Azi_PathNode` (`self.PathInfo`)))
  (return (+ _cost_g _cost_h (`self.ExtraCost`))))

(fn `GetCost_G`
  (returns (Cost :type Integer))
  (return (`.Cost_G_8_8C9147744E3021F034C64A83993FB55A` (break `/Game/Blueprints/Building/Tiles/S_Azi_PathNode` (`self.PathInfo`)))))

(fn `GetCost_H`
  (returns (Cost :type Integer))
  (return (`.Cost_H_10_A007C7D5403A6C0ACF1C6DAA63BDB9C8` (break `/Game/Blueprints/Building/Tiles/S_Azi_PathNode` (`self.PathInfo`)))))

(fn `GetParentNode`
  (returns (OutParent :type "/Game/Blueprints/Building/Tiles/BP_Tile Object Reference"))
  (return (`.Parent_5_18AA00064DF9CEEF9C305EA6CD1BE030` (break `/Game/Blueprints/Building/Tiles/S_Azi_PathNode` (`self.PathInfo`)))))

(fn `GetTraceStartLocation`
  (returns (OutLocation :type "Vector Structure"))
  (return (+ (`self.K2_GetActorLocation`) (* (`self.GetActorUpVector`) 50.0))))

(fn `Initialize`
  (params (InType :type "/Game/Blueprints/EGridType Enum" :default "NewEnumerator0"))
  (`self.SetMesh` InType)
  (bind _outlocation (`self.CalculateLocation` (`local.InType`)))
  (`self.K2_SetActorLocation` _outlocation)
  (`self.SetActorHiddenInGame` true))

(fn `IsWalkable`
  (params (InType :type "/Game/Blueprints/EGridType Enum" :default "NewEnumerator0"))
  (returns (bOutWalkable :type Boolean))
  (switch `/Game/Blueprints/EGridType` InType
    (:`NewEnumerator0`
      (return (and (not (`self.bForceNoWalkable`)) (not (`self.TraceOnBox`)))))
    (:`NewEnumerator1`
      (return (and (not (`self.bForceNoWalkable`)) (not (`self.TraceOnHexagon` true)))))
    (:`NewEnumerator2`
      (return (and (not (`self.bForceNoWalkable`)) (not (`self.TraceOnHexagon` false)))))))

(fn `OnInteract`
  (params (InColorMode :type "/Game/Blueprints/Building/Tiles/E_Azi_Colors Enum" :default "NewEnumerator0"))
  (returns (bSucess :type Boolean))
  (bind _mid (`self.MID`)
    (:`then`
      (`MaterialInstanceDynamic.SetVectorParameterValue` _mid "Color" (select `/Game/Blueprints/Building/Tiles/E_Azi_Colors` InColorMode :`NewEnumerator0` (`self.NormalColor`) :`NewEnumerator1` (`self.SelectedColor`) :`NewEnumerator2` (`self.PathColor`) :`NewEnumerator3` (`self.UnionSrcColor`) :`NewEnumerator4` (`self.UnionDstColor`)))
      (return true))
    (:`else`
      (return false))))

(fn `SetCost_G`
  (params (InCost :type Integer))
  (setmembers `/Game/Blueprints/Building/Tiles/S_Azi_PathNode` :`StructRef` (`self.PathInfo`) :`Cost_G` (+ InCost (`self.ExtraCost`))))

(fn `SetCost_H`
  (params (InCost :type Integer))
  (setmembers `/Game/Blueprints/Building/Tiles/S_Azi_PathNode` :`StructRef` (`self.PathInfo`) :`Cost_H` InCost))

(fn `SetMesh`
  (params (InType :type "/Game/Blueprints/EGridType Enum" :default "NewEnumerator0"))
  (`StaticMeshComponent.SetStaticMesh` (`self.Tile`) (select `/Game/Blueprints/EGridType` InType :`NewEnumerator0` "/Game/Blueprints/Assets/Meshes/plane.plane" :`NewEnumerator1` "/Game/Blueprints/Assets/Meshes/hexagon_P_top.hexagon_P_top" :`NewEnumerator2` "/Game/Blueprints/Assets/Meshes/hexagon_F_top.hexagon_F_top" :!type "StaticMesh Object Reference"))
  (`self.CreateMID`))

(fn `SetNeighborColor`
  (bind _mid (`self.MID`)
    (:`then`
      (`MaterialInstanceDynamic.SetVectorParameterValue` _mid "Color" (`self.PathColor`)))
    (:`else`)))

(fn `SetParentNode`
  (params (InParent :type "/Game/Blueprints/Building/Tiles/BP_Tile Object Reference"))
  (setmembers `/Game/Blueprints/Building/Tiles/S_Azi_PathNode` :`StructRef` (`self.PathInfo`) :`Parent` InParent))

(fn `TraceOnBox`
  (returns (bSuccess :type Boolean) (OutHit :type "HitResult Structure"))
  (bind _tile (`self.Tile`))
  (bind (_outhit _returnvalue) (`KismetSystemLibrary.BoxTraceSingle` (`self.GetTraceStartLocation`) (`self.K2_GetActorLocation`) (* (+ (`.BoxExtent` (`KismetSystemLibrary.GetComponentBounds` _tile)) (* (`SceneComponent.GetUpVector` _tile) 30.0)) 0.5) (struct) "TraceTypeQuery4" false (`|MakeArray` self :!type "Actor Object Reference")))
  (return _returnvalue _outhit))

(fn `TraceOnHexagon`
  (params (bInPointTop :type Boolean))
  (returns (bSuccess :type Boolean) (OutHit :type "HitResult Structure"))
  (locals (Radious :type "Float (double-precision)" :default 0.0))
  (bind (_returnvalue_x _returnvalue_y _returnvalue_z) (`KismetMathLibrary.BreakVector` (`self.GetActorUpVector`)))
  (bind _x (.x (`.BoxExtent` (`KismetSystemLibrary.GetComponentBounds` (`self.Tile`)))))
  (if (< _returnvalue_z -0.5)
    (set `local.Radious` (`KismetMathLibrary.SelectFloat` _x (.y (`.BoxExtent` (`KismetSystemLibrary.GetComponentBounds` (`self.Tile`)))) (`local.bInPointTop`)) :!label _label)
    (elif (> _returnvalue_z 0.5)
      (goto _label)
      (else
        (if (< _returnvalue_y -0.5)
          _
          (elif (> _returnvalue_y 0.5)
            _
            (else
              (goto _label))))
        (set `local.Radious` (`KismetMathLibrary.SelectFloat` _x (.z (`.BoxExtent` (`KismetSystemLibrary.GetComponentBounds` (`self.Tile`)))) (`local.bInPointTop`))))))
  (`KismetSystemLibrary.CapsuleTraceSingle` (`self.GetTraceStartLocation`) (`self.K2_GetActorLocation`) (* (`local.Radious`) 0.9) 30.0 "TraceTypeQuery4")
  (return false))

(fn `UpdateColor`
  (if (`self.bForceNoWalkable`)
    (set `self.NormalColor` (`self.DisableColor`))
    (else
      (set `self.NormalColor` (/ (`self.NormalColor`) (+ (/ (`self.ExtraCost`) 10) 1.0)))))
  (bind _returnvalue (`PrimitiveComponent.CreateDynamicMaterialInstance` (`self.Tile`) 0 "/Game/Materials/Tiles/Materials/M_Tile.M_Tile" "None"))
  (bind _output_get (set `self.MID` _returnvalue))
  (`MaterialInstanceDynamic.SetVectorParameterValue` _output_get "Color" (`self.NormalColor`)))

(fn `UserConstructionScript`
  (`TextRenderComponent.K2_SetText` (`self.TXT_Coordinates`) (`KismetTextLibrary.Conv_StringToText` (`KismetSystemLibrary.GetDisplayName` self))))