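; Multi-level navigation grid manager that spawns and attaches one BP_NavGrid per depth level of MapSize, stacked vertically at fixed spacing.
; It forwards path finding, making, deactivation and color updates to those grids.
; Paths between grids use validated NavGridsLink tile pairs for a single hop, carrying each leg's cost into the next link's search and signaling both link tiles on success.
; Player controller bindings in the event graph are unconnected.
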(event `self.ReceiveBeginPlay`)

(fn `ClearGrids`
  (bind _navgrids (`self.NavGrids`))
  (if (> (`KismetArrayLibrary.Array_Length` (`self.NavGrids`)) 0)
    (bind (_arrayindex _arrayelement) (`/Engine/EditorBlueprintResources/StandardMacros.ReverseForEachLoop` _navgrids)
      (:`LoopBody`
        (`/Game/Blueprints/Building/Grid/BP_NavGrid.ClearGridTiles` _arrayelement)
        (`self.K2_DestroyActor` _arrayelement))
      (:`Completed`
        (`KismetArrayLibrary.Array_Clear` _navgrids)))))

(fn `InitializeGrids`
  (bind (_mapsize_row _mapsize_column _mapsize_depth) (break `/Game/Blueprints/Building/Tiles/S_Azi_Coordinate` (`self.MapSize`)))
  (`self.ClearGrids`)
  (for _ (range _mapsize_depth)
    (bind _returnvalue (`|SpawnActorFromClass` "/Game/Blueprints/Building/Grid/BP_NavGrid.BP_NavGrid_C" (`KismetMathLibrary.MakeTransform` (`self.K2_GetActorLocation`) (`self.K2_GetActorRotation`)) "AlwaysSpawn" "MultiplyWithRoot" self (`self.MapSize`) (`self.Type`) null))
    (`self.K2_AttachToActor` _returnvalue self "None" "SnapToTarget" "SnapToTarget" "KeepRelative" false)
    (`/Game/Blueprints/Building/Grid/BP_NavGrid.InitializeNavGrid` _returnvalue)
    (bind _returnvalue_2 (`KismetArrayLibrary.Array_Add` (`self.NavGrids`) _returnvalue))
    (bind (_returnvalue_x _returnvalue_y _returnvalue_z) (`KismetMathLibrary.BreakVector` (`self.K2_GetActorLocation` _returnvalue)))
    (`self.K2_SetActorLocation` _returnvalue (`KismetMathLibrary.MakeVector` _returnvalue_x _returnvalue_y (+ (* _returnvalue_2 100) _returnvalue_z)) false false)))

(fn `NavGridDeactivatePath`
  (for _array_element (`self.NavGrids`)
    (`/Game/Blueprints/Building/Grid/BP_NavGrid.DeactivatePath` _array_element)))

(fn `NavGridFindPath`
  (params (InPath :type "/Game/Blueprints/Building/PathFinding/S_Azi_PathInfo Structure"))
  (locals (StartTile :type "/Game/Blueprints/Building/Tiles/BP_Tile Object Reference") (TargetTile :type "/Game/Blueprints/Building/Tiles/BP_Tile Object Reference") (OpenNodes :type "Array of /Game/Blueprints/Building/Tiles/BP_Tile Object Reference") (ClosedNodes :type "Array of /Game/Blueprints/Building/Tiles/BP_Tile Object Reference") (CurrentNode :type "/Game/Blueprints/Building/Tiles/BP_Tile Object Reference") (Neightbors :type "Array of /Game/Blueprints/Building/Tiles/BP_Tile Object Reference") (NeightborNode :type "/Game/Blueprints/Building/Tiles/BP_Tile Object Reference"))
  (for _array_element (`self.NavGrids`)
    (`/Game/Blueprints/Building/Grid/BP_NavGrid.FindPath` _array_element InPath)))

(fn `NavGridFindPathTo`
  (params (InStart :type "Actor Object Reference") (InTarget :type "Actor Object Reference") (InTargetActor :type "Actor Object Reference"))
  (locals (LocalStartNavGrid :type "/Game/Blueprints/Building/Grid/BP_NavGrid Object Reference") (LocalStartTile :type "/Game/Blueprints/Building/Tiles/BP_Tile Object Reference") (LocalEndNavGrid :type "/Game/Blueprints/Building/Grid/BP_NavGrid Object Reference") (LocalEndTile :type "/Game/Blueprints/Building/Tiles/BP_Tile Object Reference") (LocalStartTile2nd :type "/Game/Blueprints/Building/Tiles/BP_Tile Object Reference") (LocalEndTile2nd :type "/Game/Blueprints/Building/Tiles/BP_Tile Object Reference") (LocalStartNavGrid2nd :type "/Game/Blueprints/Building/Grid/BP_NavGrid Object Reference") (LastCostA :type Integer :default -1) (LastCostB :type Integer :default -1))
  (bind _returnvalue (`self.GetOwner` InStart))
  (`/Engine/EditorBlueprintResources/StandardMacros.IsValid` InTargetActor
    (:`Is Valid`
      (if (== _returnvalue (`self.GetOwner` InTarget))
        (bind _asbp_nav_grid (cast `/Game/Blueprints/Building/Grid/BP_NavGrid` _returnvalue))
        (for _array_element (`self.NavGrids`)
          (if (== _array_element _asbp_nav_grid)
            (`/Game/Blueprints/Building/Grid/BP_NavGrid.FindPathTo` _array_element (`local.InStart`) (`local.InTarget`) (`local.InTargetActor`) -1)))
        (else
          (for _array_element_2 (`self.NavGridsLink`)
            (bind _outisvalid (`self.NavGridIsTileValid` _array_element_2))
            (if _outisvalid
              (bind (_startnavgrid _starttile _endnavgrid _endtile) (break `/Game/Blueprints/Building/Tiles/S_Azi_NavGridLink` _array_element_2))
              (set `local.LocalStartNavGrid` _startnavgrid)
              (set `local.LocalEndNavGrid` _endnavgrid)
              (set `local.LocalStartTile` _starttile)
              (set `local.LocalEndTile` _endtile)
              (if (== (`local.LocalStartNavGrid`) (`self.GetOwner` (`local.InStart`)))
                (if (== (`local.LocalEndNavGrid`) (`self.GetOwner` (`local.InTarget`)))
                  (bind (_bsuccess _outcost) (`/Game/Blueprints/Building/Grid/BP_NavGrid.FindPathTo` (`local.LocalStartNavGrid`) (`local.InStart`) (`local.LocalStartTile`) (`local.InTargetActor`) (`local.LastCostA`)))
                  (if _bsuccess
                    (set `local.LastCostA` _outcost)
                    (bind (_bsuccess_2 _outcost_2) (`/Game/Blueprints/Building/Grid/BP_NavGrid.FindPathTo` (`local.LocalEndNavGrid`) (`local.LocalEndTile`) (`local.InTarget`) null (`local.LastCostB`)))
                    (if _bsuccess_2
                      (set `local.LastCostB` _outcost_2)
                      (message `/Game/Blueprints/Libraries/BPI_interactable.OnInteract` (`local.LocalStartTile`) "NewEnumerator3")
                      (message `/Game/Blueprints/Libraries/BPI_interactable.OnInteract` (`local.LocalEndTile`) "NewEnumerator4"))))))))))))

(fn `NavGridIsTileValid`
  (params (InNavGridLink :type "/Game/Blueprints/Building/Tiles/S_Azi_NavGridLink Structure"))
  (returns (OutIsValid :type Boolean))
  (bind (_startnavgrid _starttile _endnavgrid _endtile) (break `/Game/Blueprints/Building/Tiles/S_Azi_NavGridLink` InNavGridLink))
  (`/Engine/EditorBlueprintResources/StandardMacros.IsValid` _startnavgrid
    (:`Is Valid`
      (if (== _startnavgrid (`self.GetOwner` _starttile))
        (`/Engine/EditorBlueprintResources/StandardMacros.IsValid` _endnavgrid
          (:`Is Valid`
            (if (== _endnavgrid (`self.GetOwner` _endtile))
              (return true)
              (else
                (return false))))
          (:`Is Not Valid`
            (return false)))
        (else
          (return false))))
    (:`Is Not Valid`
      (return false))))

(fn `NavGridMakePath`
  (params (InStart :type "/Game/Blueprints/Building/Tiles/BP_Tile Object Reference") (InTarget :type "/Game/Blueprints/Building/Tiles/BP_Tile Object Reference"))
  (locals (CurrentNode :type "/Game/Blueprints/Building/Tiles/BP_Tile Object Reference") (Result :type "Array of /Game/Blueprints/Building/Tiles/BP_Tile Object Reference"))
  (for _array_element (`self.NavGrids`)
    (`/Game/Blueprints/Building/Grid/BP_NavGrid.MakePath` _array_element InStart InTarget)))

(fn `UpdateColors`
  (for _array_element (`self.NavGrids`)
    (`/Game/Blueprints/Building/Grid/BP_NavGrid.UpdateColors` _array_element)))

(fn `UserConstructionScript`)