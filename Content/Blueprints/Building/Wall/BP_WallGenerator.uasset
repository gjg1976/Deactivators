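; Wall generator actor that builds a building wall from a row-by-column grid of attached BP_WallTile actors.
; InitializeWall clears the previous wall, spawns indexed tiles and adds optional horizontal or vertical BP_WallBorder pieces placed by actor bounds.
; MakeHole rebuilds without borders at a zero transform, restores the transform, then destroys tiles flagged in HoleMap.
; Helpers apply materials with a shared random value, hide tiles and look up grid neighbors.
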(event `self.ReceiveBeginPlay`
  (for _array_element _
    (if (`/Game/Blueprints/Building/Tiles/BP_Tile.IsWalkable` _array_element "NewEnumerator0")
      _)))

(fn `AddBorderLeft`
  (bind (_returnvalue_x _returnvalue_y _returnvalue_z) (`KismetMathLibrary.BreakVector` (`self.K2_GetActorLocation`)))
  (bind _mapsize_row (break `/Game/Blueprints/Building/Tiles/S_Azi_Coordinate` (`self.MapSize`)))
  (for _index (range _mapsize_row)
    (bind _returnvalue (`|SpawnActorFromClass` "/Game/Blueprints/Building/Tiles/BP_WallBorder.BP_WallBorder_C" (`KismetMathLibrary.MakeTransform` (`self.K2_GetActorLocation`) (`self.K2_GetActorRotation`)) "AlwaysSpawn" "MultiplyWithRoot" self (make `/Game/Blueprints/Building/Tiles/S_Azi_Coordinate` _index) null))
    (`self.K2_AttachToActor` _returnvalue self "None" "SnapToTarget" "SnapToTarget" "KeepRelative" false)
    (bind (_origin _boxextent) (`self.GetActorBounds` _returnvalue false false))
    (`/Game/Blueprints/Building/Tiles/BP_WallBorder.Initialize` _returnvalue 0 (`KismetMathLibrary.MakeVector` (- _returnvalue_x (.x _boxextent)) (+ _returnvalue_y (.y _boxextent) (* (.y _boxextent) _index 2.0)) (+ _returnvalue_z (.z _boxextent))))
    (`KismetArrayLibrary.Array_Add` (`self.TileBorders`) _returnvalue)))

(fn `AddBorderLower`
  (bind (_returnvalue_x _returnvalue_y _returnvalue_z) (`KismetMathLibrary.BreakVector` (`self.K2_GetActorLocation`)))
  (bind _mapsize_row (break `/Game/Blueprints/Building/Tiles/S_Azi_Coordinate` (`self.MapSize`)))
  (bind _mapsize_row_2 (break `/Game/Blueprints/Building/Tiles/S_Azi_Coordinate` (`self.MapSize`)))
  (for _index (range _mapsize_row)
    (bind _returnvalue (`|SpawnActorFromClass` "/Game/Blueprints/Building/Tiles/BP_WallBorder.BP_WallBorder_C" (`KismetMathLibrary.MakeTransform` (`self.K2_GetActorLocation`) (`self.K2_GetActorRotation`)) "AlwaysSpawn" "MultiplyWithRoot" self (make `/Game/Blueprints/Building/Tiles/S_Azi_Coordinate` _index) null))
    (`self.K2_AttachToActor` _returnvalue self "None" "SnapToTarget" "SnapToTarget" "KeepRelative" false)
    (`self.K2_SetActorRelativeRotation` _returnvalue (struct :`Yaw` -90.0) false false)
    (bind (_origin _boxextent) (`self.GetActorBounds` _returnvalue false false))
    (`/Game/Blueprints/Building/Tiles/BP_WallBorder.Initialize` _returnvalue 0 (`KismetMathLibrary.MakeVector` (+ _returnvalue_x (* _index (.x _boxextent) 2.0) (.x _boxextent)) (+ _returnvalue_y (* (.y (`.BoxExtent` (`self.GetActorBounds` (`|GetArrayItem` (`self.Tiles`)) false false))) 2.0 _mapsize_row_2) (.y _boxextent)) (+ _returnvalue_z (.z _boxextent))))
    (`KismetArrayLibrary.Array_Add` (`self.TileBorders`) _returnvalue)))

(fn `AddBorderRight`
  (bind (_returnvalue_x _returnvalue_y _returnvalue_z) (`KismetMathLibrary.BreakVector` (`self.K2_GetActorLocation`)))
  (bind _mapsize_row (break `/Game/Blueprints/Building/Tiles/S_Azi_Coordinate` (`self.MapSize`)))
  (bind (_mapsize_row_2 _mapsize_column) (break `/Game/Blueprints/Building/Tiles/S_Azi_Coordinate` (`self.MapSize`)))
  (for _index (range _mapsize_row)
    (bind _returnvalue (`|SpawnActorFromClass` "/Game/Blueprints/Building/Tiles/BP_WallBorder.BP_WallBorder_C" (`KismetMathLibrary.MakeTransform` (`self.K2_GetActorLocation`) (`self.K2_GetActorRotation`)) "AlwaysSpawn" "MultiplyWithRoot" self (make `/Game/Blueprints/Building/Tiles/S_Azi_Coordinate` _index) null))
    (`self.K2_AttachToActor` _returnvalue self "None" "SnapToTarget" "SnapToTarget" "KeepRelative" false)
    (`/Engine/EditorBlueprintResources/StandardMacros.IsValid` (`|GetArrayItem` (`self.Tiles`))
      (:`Is Valid`
        (bind (_origin _boxextent) (`self.GetActorBounds` _returnvalue false false))
        (`/Game/Blueprints/Building/Tiles/BP_WallBorder.Initialize` _returnvalue 0 (`KismetMathLibrary.MakeVector` (+ _returnvalue_x (.x _boxextent) (* (.x (`.BoxExtent` (`self.GetActorBounds` (`|GetArrayItem` (`self.Tiles`)) false false))) 2.0 _mapsize_column)) (+ _returnvalue_y (.y _boxextent) (* (.y _boxextent) _index 2.0)) (+ _returnvalue_z (.z _boxextent))))
        (`KismetArrayLibrary.Array_Add` (`self.TileBorders`) _returnvalue)))))

(fn `AddBorderUpper`
  (bind (_returnvalue_x _returnvalue_y _returnvalue_z) (`KismetMathLibrary.BreakVector` (`self.K2_GetActorLocation`)))
  (bind _mapsize_row (break `/Game/Blueprints/Building/Tiles/S_Azi_Coordinate` (`self.MapSize`)))
  (for _index (range _mapsize_row)
    (bind _returnvalue (`|SpawnActorFromClass` "/Game/Blueprints/Building/Tiles/BP_WallBorder.BP_WallBorder_C" (`KismetMathLibrary.MakeTransform` (`self.K2_GetActorLocation`) (`self.K2_GetActorRotation`)) "AlwaysSpawn" "MultiplyWithRoot" self (make `/Game/Blueprints/Building/Tiles/S_Azi_Coordinate` _index) null))
    (`self.K2_AttachToActor` _returnvalue self "None" "SnapToTarget" "SnapToTarget" "KeepRelative" false)
    (`self.K2_SetActorRelativeRotation` _returnvalue (struct :`Yaw` -90.0) false false)
    (bind (_origin _boxextent) (`self.GetActorBounds` _returnvalue false false))
    (`/Game/Blueprints/Building/Tiles/BP_WallBorder.Initialize` _returnvalue 0 (`KismetMathLibrary.MakeVector` (+ _returnvalue_x (* _index (.x _boxextent) 2.0) (.x _boxextent)) (- _returnvalue_y (.y _boxextent)) (+ _returnvalue_z (.z _boxextent))))
    (`KismetArrayLibrary.Array_Add` (`self.TileBorders`) _returnvalue)))

(fn `ChangeMaterial`
  (params (InWallID :type "/Game/Blueprints/Building/Wall/E_Dea_WallID Enum" :default "NewEnumerator0"))
  (locals (RandomNum :type Integer :default 0))
  (set `local.RandomNum` (`KismetMathLibrary.RandomInteger` 9))
  (for _array_element (`self.Tiles`)
    (`/Game/Blueprints/Building/Tiles/BP_WallTile.CreateMID` _array_element (`local.InWallID`) (`local.RandomNum`)))
  (for _array_element_2 (`self.TileBorders`)
    (`/Game/Blueprints/Building/Tiles/BP_WallBorder.CreateMID` _array_element_2 (`local.InWallID`) (`local.RandomNum`))))

(fn `ClearWall`
  (bind _tileborders (`self.TileBorders`))
  (bind _tiles (`self.Tiles`))
  (if (> (`KismetArrayLibrary.Array_Length` (`self.Tiles`)) 0)
    (bind (_arrayindex _arrayelement) (`/Engine/EditorBlueprintResources/StandardMacros.ReverseForEachLoop` _tiles)
      (:`LoopBody`
        (`/Game/Blueprints/Building/Tiles/BP_WallTile.ClearDecoration` _arrayelement)
        (`self.K2_DestroyActor` _arrayelement))
      (:`Completed`
        (`KismetArrayLibrary.Array_Clear` _tiles)
        (bind (_arrayindex_2 _arrayelement_2) (`/Engine/EditorBlueprintResources/StandardMacros.ReverseForEachLoop` _tileborders)
          (:`LoopBody`
            (`self.K2_DestroyActor` _arrayelement_2))
          (:`Completed`
            (`KismetArrayLibrary.Array_Clear` _tileborders)))))))

(fn `GetBound`
  (returns (Bound :type "Vector Structure"))
  (bind _output (`|GetArrayItem` (`self.Tiles`)))
  (`/Engine/EditorBlueprintResources/StandardMacros.IsValid` _output
    (:`Is Valid`
      (return (`KismetMathLibrary.MakeVector` (* (.x (`/Game/Blueprints/Building/Tiles/BP_WallTile.GetBound` _output)) 4.0) (* (.y (`/Game/Blueprints/Building/Tiles/BP_WallTile.GetBound` _output)) 4.0) (.z (`/Game/Blueprints/Building/Tiles/BP_WallTile.GetBound` _output)))))
    (:`Is Not Valid`
      (return (0.0 0.0 0.0)))))

(fn `GetNeighbor`
  (params (InId :type Integer) (InCoordinate :type "/Game/Blueprints/Building/Tiles/S_Azi_Coordinate Structure") (InDirection :type "/Game/Blueprints/Building/Tiles/E_Azi_Direction Enum" :default "NewEnumerator0"))
  (returns (OutNeighbor :type "/Game/Blueprints/Building/Tiles/BP_WallTile Object Reference"))
  (bind (_incoordinate_row _incoordinate_column) (break `/Game/Blueprints/Building/Tiles/S_Azi_Coordinate` (`local.InCoordinate`)))
  (bind (_mapsize_row _mapsize_column) (break `/Game/Blueprints/Building/Tiles/S_Azi_Coordinate` (`self.MapSize`)))
  (bind (_mapsize_row_2 _mapsize_column_2) (break `/Game/Blueprints/Building/Tiles/S_Azi_Coordinate` (`self.MapSize`)))
  (bind (_incoordinate_row_2 _incoordinate_column_2) (break `/Game/Blueprints/Building/Tiles/S_Azi_Coordinate` (`local.InCoordinate`)))
  (bind (_incoordinate_row_3 _incoordinate_column_3) (break `/Game/Blueprints/Building/Tiles/S_Azi_Coordinate` (`local.InCoordinate`)))
  (bind _mapsize_row_3 (break `/Game/Blueprints/Building/Tiles/S_Azi_Coordinate` (`self.MapSize`)))
  (bind (_mapsize_row_4 _mapsize_column_3) (break `/Game/Blueprints/Building/Tiles/S_Azi_Coordinate` (`self.MapSize`)))
  (bind (_incoordinate_row_4 _incoordinate_column_4) (break `/Game/Blueprints/Building/Tiles/S_Azi_Coordinate` (`local.InCoordinate`)))
  (bind (_mapsize_row_5 _mapsize_column_4) (break `/Game/Blueprints/Building/Tiles/S_Azi_Coordinate` (`self.MapSize`)))
  (bind (_mapsize_row_6 _mapsize_column_5) (break `/Game/Blueprints/Building/Tiles/S_Azi_Coordinate` (`self.MapSize`)))
  (bind (_incoordinate_row_5 _incoordinate_column_5) (break `/Game/Blueprints/Building/Tiles/S_Azi_Coordinate` (`local.InCoordinate`)))
  (bind (_mapsize_row_7 _mapsize_column_6) (break `/Game/Blueprints/Building/Tiles/S_Azi_Coordinate` (`self.MapSize`)))
  (bind (_incoordinate_row_6 _incoordinate_column_6) (break `/Game/Blueprints/Building/Tiles/S_Azi_Coordinate` (`local.InCoordinate`)))
  (bind (_incoordinate_row_7 _incoordinate_column_7) (break `/Game/Blueprints/Building/Tiles/S_Azi_Coordinate` (`local.InCoordinate`)))
  (bind (_mapsize_row_8 _mapsize_column_7) (break `/Game/Blueprints/Building/Tiles/S_Azi_Coordinate` (`self.MapSize`)))
  (bind (_mapsize_row_9 _mapsize_column_8) (break `/Game/Blueprints/Building/Tiles/S_Azi_Coordinate` (`self.MapSize`)))
  (bind (_incoordinate_row_8 _incoordinate_column_8) (break `/Game/Blueprints/Building/Tiles/S_Azi_Coordinate` (`local.InCoordinate`)))
  (bind _incoordinate_row_9 (break `/Game/Blueprints/Building/Tiles/S_Azi_Coordinate` (`local.InCoordinate`)))
  (bind (_incoordinate_row_10 _incoordinate_column_9) (break `/Game/Blueprints/Building/Tiles/S_Azi_Coordinate` (`local.InCoordinate`)))
  (bind (_mapsize_row_10 _mapsize_column_9) (break `/Game/Blueprints/Building/Tiles/S_Azi_Coordinate` (`self.MapSize`)))
  (bind (_incoordinate_row_11 _incoordinate_column_10) (break `/Game/Blueprints/Building/Tiles/S_Azi_Coordinate` (`local.InCoordinate`)))
  (bind _returnvalue (* (- _incoordinate_row_11 (`KismetMathLibrary.SelectInt` 1 0 (== (mod _incoordinate_column_10 2) 0))) _mapsize_column_3))
  (if (> InId -1)
    (switch `/Game/Blueprints/Building/Tiles/E_Azi_Direction` (`local.InDirection`)
      (:`NewEnumerator0`
        ; North Neighbors
        (if true
          (if (> _incoordinate_row 0)
            (return (`|GetArrayItem` (`self.Tiles`) (+ _incoordinate_column (* (- _incoordinate_row 1) _mapsize_column))))
            (else
              (return null)))
          (else
            (return null))))
      (:`NewEnumerator1`
        ; East Neighbors
        (if true
          (if (< _incoordinate_column_4 (- _mapsize_column_5 1))
            (return (`|GetArrayItem` (`self.Tiles`) (+ _incoordinate_column_4 1 (* _incoordinate_row_4 _mapsize_column_4))))
            (else
              (return null)))
          (else
            (return null))))
      (:`NewEnumerator2`
        ; South Neighbors
        (if true
          (if (< _incoordinate_row_2 (- _mapsize_row_3 1))
            (return (`|GetArrayItem` (`self.Tiles`) (+ _incoordinate_column_2 (* (+ _incoordinate_row_2 1) _mapsize_column_2))))
            (else
              (return null)))
          (else
            (return null))))
      (:`NewEnumerator3`
        ; west Neighbors
        (if true
          (if (> _incoordinate_column_5 0)
            (return (`|GetArrayItem` (`self.Tiles`) (+ (- _incoordinate_column_5 1) (* _incoordinate_row_5 _mapsize_column_6))))
            (else
              (return null)))
          (else
            (return null))))
      (:`NewEnumerator4`
        ; NorthEast Neighbor
        (switch `/Game/Blueprints/EGridType` "NewEnumerator0"
          (:`NewEnumerator0`
            (if (and (> _incoordinate_row_7 0) (< _incoordinate_column_7 (- _mapsize_column_7 1)))
              (return (`|GetArrayItem` (`self.Tiles`) (- (`local.InId`) (- _mapsize_column_8 1))))
              (else
                (return null))))
          (:`NewEnumerator1`
            (if (> _incoordinate_row_9 0)
              (if (not (or (< _incoordinate_column_9 (- _mapsize_column_9 1)) (== (mod _incoordinate_row_10 2) 0)))
                (return null))
              (else
                (return null))))
          (:`NewEnumerator2`
            (if (< _incoordinate_column_3 (- _incoordinate_column_8 1))
              (if (> _returnvalue -1)
                (return (`|GetArrayItem` (`self.Tiles`) (+ _returnvalue 1 _incoordinate_column_6)))
                (else
                  (return null)))
              (else
                (return null)))))))
    (else
      (return null))))

(fn `GetTileId`
  (params (InTile :type "/Game/Blueprints/Building/Tiles/BP_WallTile Object Reference"))
  (returns (OutId :type Integer))
  (bind (_mapsize_row _mapsize_column) (break `/Game/Blueprints/Building/Tiles/S_Azi_Coordinate` (`self.MapSize`)))
  (bind (_coordinate_row _coordinate_column) (break `/Game/Blueprints/Building/Tiles/S_Azi_Coordinate` (`/Game/Blueprints/Building/Tiles/BP_WallTile.Coordinate` (`local.InTile`))))
  (`/Engine/EditorBlueprintResources/StandardMacros.IsValid` InTile
    (:`Is Valid`
      (return (+ (* _coordinate_row _mapsize_column) _coordinate_column)))
    (:`Is Not Valid`
      (return -1))))

(fn `GetTileNeighbors`
  (params (InTile :type "/Game/Blueprints/Building/Tiles/BP_WallTile Object Reference") (bInDiagonally :type Boolean))
  (returns (OutNeightbors :type "Array of /Game/Blueprints/Building/Tiles/BP_WallTile Object Reference"))
  (locals (TileId :type Integer :default 0) (Result :type "Array of /Game/Blueprints/Building/Tiles/BP_WallTile Object Reference"))
  (`/Engine/EditorBlueprintResources/StandardMacros.IsValid` InTile
    (:`Is Valid`
      (bind _output_get (set `local.TileId` (`self.GetTileId` (`local.InTile`))))
      (if (> _output_get -1)
        (for _index (range (+ (`KismetMathLibrary.SelectInt` 7 3 (`local.bInDiagonally`)) 1))
          (bind _outneighbor (`self.GetNeighbor` (`local.TileId`) (`/Game/Blueprints/Building/Tiles/BP_WallTile.Coordinate` (`local.InTile`)) (cast `/Game/Blueprints/Building/Tiles/E_Azi_Direction` (`KismetMathLibrary.Conv_IntToByte` _index))))
          (`/Engine/EditorBlueprintResources/StandardMacros.IsValid` _outneighbor
            (:`Is Valid`
              (`KismetArrayLibrary.Array_Add` (`local.Result`) _outneighbor))))
        (return (`local.Result`))
        (else
          (return))))
    (:`Is Not Valid`
      (return))))

(fn `HideWall`
  (bind (_arrayindex _arrayelement) (`/Engine/EditorBlueprintResources/StandardMacros.ReverseForEachLoop` (`self.Tiles`))
    (:`LoopBody`
      (`self.SetActorHiddenInGame` _arrayelement true))))

(fn `InitializeWall`
  (params (InBorder :type "/Game/Blueprints/Building/Wall/E_Dea_WallBorders Enum" :default "NewEnumerator7"))
  (bind (_mapsize_row _mapsize_column) (break `/Game/Blueprints/Building/Tiles/S_Azi_Coordinate` (`self.MapSize`)))
  (bind (_mapsize_row_2 _mapsize_column_2) (break `/Game/Blueprints/Building/Tiles/S_Azi_Coordinate` (`self.MapSize`)))
  (`self.ClearWall`)
  (for _index (range _mapsize_row)
    (for _index_2 (range _mapsize_column)
      (bind _returnvalue (`|SpawnActorFromClass` "/Game/Blueprints/Building/Tiles/BP_WallTile.BP_WallTile_C" (`KismetMathLibrary.MakeTransform` (`self.K2_GetActorLocation`) (`self.K2_GetActorRotation`)) "AlwaysSpawn" "MultiplyWithRoot" self (make `/Game/Blueprints/Building/Tiles/S_Azi_Coordinate` _index _index_2) null))
      (`self.K2_AttachToActor` _returnvalue self "None" "SnapToTarget" "SnapToTarget" "KeepRelative" false)
      (`/Game/Blueprints/Building/Tiles/BP_WallTile.Initialize` _returnvalue (+ _index_2 (* _index _mapsize_column_2)))
      (`KismetArrayLibrary.Array_Add` (`self.Tiles`) _returnvalue)))
  (switch `/Game/Blueprints/Building/Wall/E_Dea_WallBorders` (`local.InBorder`)
    (:`NewEnumerator8`
      (`self.AddBorderRight`)
      (`self.AddBorderLeft`))
    (:`NewEnumerator9`
      (`self.AddBorderUpper`)
      (`self.AddBorderLower`))
    (:`NewEnumerator10`
      (`self.AddBorderRight`)
      (`self.AddBorderLeft`)
      (`self.AddBorderUpper`)
      (`self.AddBorderLower`))))

(fn `MakeHole`
  (bind (_returnvalue_location _returnvalue_rotation) (`KismetMathLibrary.BreakTransform` (`self.GetTransform`)))
  (set `self.Location` _returnvalue_location)
  (set `self.Rotation` _returnvalue_rotation)
  (`KismetArrayLibrary.Array_Clear` (`self.TilesToRemove`))
  (`self.K2_SetActorLocationAndRotation` (0.0 0.0 0.0))
  (`self.InitializeWall` "NewEnumerator7")
  (`self.K2_SetActorLocationAndRotation` (`self.Location`) (`self.Rotation`))
  (`|ExecutionSequence`
    (:`then_0`
      (for (_array_element _array_index) (`self.Tiles`)
        (`/Engine/EditorBlueprintResources/StandardMacros.IsValid` _array_element
          (:`Is Valid`
            (if (`|GetArrayItem` (`self.HoleMap`) _array_index)
              (`KismetArrayLibrary.Array_Add` (`self.TilesToRemove`) _array_element))))))
    (:`then_1`
      (for _array_element_2 (`self.TilesToRemove`)
        (`KismetArrayLibrary.Array_RemoveItem` (`self.Tiles`) _array_element_2)
        (`self.K2_DestroyActor` _array_element_2)))))

(fn `UserConstructionScript`)