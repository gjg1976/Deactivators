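; BP_RoomGravity is a room volume that gives overlapping actors one of four directional gravities, set by compass direction and a strength value.
; Each Tick it sets CharacterMovement gravity direction on Guardians, also done at BeginPlay, and adds mass-scaled force to bomb and circuit board meshes.
; GetGravityVector maps North/South to vertical and East/West to the Y axis.
; ApplyGravityToActor offers per-actor application, including Deactivators, but is not called here.
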(event `self.ReceiveTick`
  (params (DeltaSeconds :type "Float (single-precision)"))
  (for _array_element (`self.GetOverlappingActors` "/Game/Blueprints/Assets/BP_Guardian.BP_Guardian_C")
    (bind _asbp_guardian (cast `/Game/Blueprints/Assets/BP_Guardian` _array_element))
    (`CharacterMovementComponent.SetGravityDirection` (`Character.CharacterMovement` _asbp_guardian) (`self.GetGravityVector`)))
  (for _array_element_2 (`self.GetOverlappingActors` "/Game/Blueprints/Assets/BP_CircuitBoard.BP_CircuitBoard_C")
    (`self.ApplyGravityToCircuitBoard` _array_element_2))
  (for _array_element_3 (`self.GetOverlappingActors` "/Game/Blueprints/Assets/BP_bomb.BP_bomb_C")
    (`self.ApplyGravityToBomb` _array_element_3)))

(event `self.ReceiveBeginPlay`
  (for _array_element (`self.GetOverlappingActors` "/Game/Blueprints/Assets/BP_Guardian.BP_Guardian_C")
    (bind _asbp_guardian (cast `/Game/Blueprints/Assets/BP_Guardian` _array_element))
    (`CharacterMovementComponent.SetGravityDirection` (`Character.CharacterMovement` _asbp_guardian) (`self.GetGravityVector`))))

(fn `ApplyGravityToActor`
  (params (InActor :type "Actor Object Reference"))
  (bind _asbp_deactivator_3 (cast `/Game/PortalSystem/DemoContent/ThirdPersonBP/Blueprints/BP_Deactivator3` InActor)
    (:`then`
      (`CharacterMovementComponent.SetGravityDirection` (`Character.CharacterMovement` _asbp_deactivator_3) (`self.GetGravityVector`)))
    (:`CastFailed`
      (bind _asbp_guardian (cast `/Game/Blueprints/Assets/BP_Guardian` (`local.InActor`))
        (:`then`
          (`CharacterMovementComponent.SetGravityDirection` (`Character.CharacterMovement` _asbp_guardian) (`self.GetGravityVector`)))
        (:`CastFailed`
          (bind _asbp_bomb (cast `/Game/Blueprints/Assets/BP_bomb` (`local.InActor`))
            (:`then`
              (`/Game/Blueprints/Assets/BP_bomb.SetGravity` _asbp_bomb (`self.GravityStreight`)))
            (:`CastFailed`
              (bind _asbp_circuit_board (cast `/Game/Blueprints/Assets/BP_CircuitBoard` (`local.InActor`)))
              (`/Game/Blueprints/Assets/BP_CircuitBoard.SetGravity` _asbp_circuit_board (`self.GravityStreight`)))))))))

(fn `ApplyGravityToBomb`
  (params (InBomb :type "/Game/Blueprints/Assets/BP_bomb Object Reference"))
  (`PrimitiveComponent.AddForce` (`/Game/Blueprints/Assets/BP_bomb.SM_Bomb` InBomb) (* (* (`PrimitiveComponent.GetMass` (`/Game/Blueprints/Assets/BP_bomb.SM_Bomb` InBomb)) 98.0 (`self.GravityStreight`)) (`self.GetGravityVector`)) "None" true))

(fn `ApplyGravityToCircuitBoard`
  (params (InCircuit :type "/Game/Blueprints/Assets/BP_CircuitBoard Object Reference"))
  (`PrimitiveComponent.AddForce` (`/Game/Blueprints/Assets/BP_CircuitBoard.SM_ComputerBoard` InCircuit) (* (* (`PrimitiveComponent.GetMass` (`/Game/Blueprints/Assets/BP_CircuitBoard.SM_ComputerBoard` InCircuit)) 98.0 (`self.GravityStreight`)) (`self.GetGravityVector`)) "None" true))

(fn `GetGravityVector`
  (returns (OutGravity :type "Vector Structure"))
  (locals (LocalGravityDirection :type "Vector Structure" :default (0.0 0.0 0.0)))
  (switch `/Game/Blueprints/Building/Room/E_Dea_RoomDirection` (`self.GravityDirection`)
    (:`NewEnumerator0`
      (set `local.LocalGravityDirection` (`KismetMathLibrary.MakeVector` 0.0 0.0 -1.0)))
    (:`NewEnumerator1`
      (set `local.LocalGravityDirection` (`KismetMathLibrary.MakeVector` 0.0 -1.0)))
    (:`NewEnumerator2`
      (set `local.LocalGravityDirection` (`KismetMathLibrary.MakeVector` 0.0 0.0 1.0)))
    (:`NewEnumerator3`
      (set `local.LocalGravityDirection` (`KismetMathLibrary.MakeVector` 0.0 1.0))))
  (return (* (`local.LocalGravityDirection`) (`self.GravityStreight`))))

(fn `Initialize`
  (set `self.GravityDirection` "NewEnumerator0")
  (set `self.GravityStreight` 1.0))

(fn `SetGravityDirection`
  (params (InGravityDirection :type "/Game/Blueprints/Building/Room/E_Dea_RoomDirection Enum" :default "NewEnumerator0"))
  (set `self.GravityDirection` InGravityDirection))

(fn `UserConstructionScript`)