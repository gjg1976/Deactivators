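; Main computer with eight circuit board slots that trigger linked actors as boards are delivered.
; On BeginPlay it shows pre-filled boards from slot 7 downward, based on FreeSlots.
; When a BP_Deactivator3 enters the trigger box, it takes and destroys its circuit board, plays a sound and adds score through BP_BuildingGenerator.
; The board's CircuitNumber picks the slot to show and the target array that receives BPI_Computer SlotTrigger calls.
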(event `self.ReceiveBeginPlay`
  (for _index (range 1 (+ (- 8 (`self.FreeSlots`)) 1))
    (switch `int` (- 8 _index)
      (:`0`
        (`SceneComponent.SetVisibility` (`self.ComputerBoard0`) true false))
      (:`1`
        (`SceneComponent.SetVisibility` (`self.ComputerBoard1`) true false))
      (:`2`
        (`SceneComponent.SetVisibility` (`self.ComputerBoard2`) true false))
      (:`3`
        (`SceneComponent.SetVisibility` (`self.ComputerBoard3`) true false))
      (:`4`
        (`SceneComponent.SetVisibility` (`self.ComputerBoard4`) true false))
      (:`5`
        (`SceneComponent.SetVisibility` (`self.ComputerBoard5`) true false))
      (:`6`
        (`SceneComponent.SetVisibility` (`self.ComputerBoard6`) true false))
      (:`7`
        (`SceneComponent.SetVisibility` (`self.ComputerBoard7`) true false)))))

(event `self.TriggerBox.OnComponentBeginOverlap`
  (params (OverlappedComponent :type "PrimitiveComponent Object Reference") (OtherActor :type "Actor Object Reference") (OtherComp :type "PrimitiveComponent Object Reference") (OtherBodyIndex :type Integer) (bFromSweep :type Boolean) (SweepResult :type "HitResult Structure (by ref)"))
  (bind _asbp_deactivator_3 (cast `/Game/PortalSystem/DemoContent/ThirdPersonBP/Blueprints/BP_Deactivator3` OtherActor))
  (bind _outcircuitboard (`/Game/PortalSystem/DemoContent/ThirdPersonBP/Blueprints/BP_Deactivator3.DetachCircuitBoard` _asbp_deactivator_3))
  (`/Engine/EditorBlueprintResources/StandardMacros.IsValid` _outcircuitboard
    (:`Is Valid`
      (set `self.Circuit Number` (`/Game/Blueprints/Assets/BP_CircuitBoard.CircuitNumber` _outcircuitboard))
      (`self.K2_DestroyActor` _outcircuitboard)
      (`GameplayStatics.PlaySound2D` "/Game/Sounds/computer.computer" 1.0 1.0 0.0 null null)
      (bind _returnvalue (`GameplayStatics.GetActorOfClass` "/Game/Blueprints/Building/BP_BuildingGenerator.BP_BuildingGenerator_C"))
      (`/Engine/EditorBlueprintResources/StandardMacros.IsValid` _returnvalue
        (:`Is Valid`
          (`/Game/Blueprints/Building/BP_BuildingGenerator.AddScore` _returnvalue "NewEnumerator0" null)
          (switch `int` (`self.Circuit Number`)
            (:`0`
              (`SceneComponent.SetVisibility` (`self.ComputerBoard0`) true false)
              (for _array_element (`self.Slot0_Target`)
                (`/Engine/EditorBlueprintResources/StandardMacros.IsValid` _array_element
                  (:`Is Valid`
                    (bind _asbpi_computer (cast `/Game/Blueprints/Libraries/BPI_Computer` _array_element))
                    (`/Game/Blueprints/Libraries/BPI_Computer.Slot_Trigger` _asbpi_computer)))))
            (:`1`
              (`SceneComponent.SetVisibility` (`self.ComputerBoard1`) true false)
              (for _array_element_2 (`self.Slot1_Target`)
                (`/Engine/EditorBlueprintResources/StandardMacros.IsValid` _array_element_2
                  (:`Is Valid`
                    (bind _asbpi_computer_2 (cast `/Game/Blueprints/Libraries/BPI_Computer` _array_element_2))
                    (`/Game/Blueprints/Libraries/BPI_Computer.Slot_Trigger` _asbpi_computer_2)))))
            (:`2`
              (`SceneComponent.SetVisibility` (`self.ComputerBoard2`) true false)
              (for _array_element_3 (`self.Slot2_Target`)
                (`/Engine/EditorBlueprintResources/StandardMacros.IsValid` _array_element_3
                  (:`Is Valid`
                    (bind _asbpi_computer_3 (cast `/Game/Blueprints/Libraries/BPI_Computer` _array_element_3))
                    (`/Game/Blueprints/Libraries/BPI_Computer.Slot_Trigger` _asbpi_computer_3)))))
            (:`3`
              (`SceneComponent.SetVisibility` (`self.ComputerBoard3`) true false)
              (for _array_element_4 (`self.Slot3_Target`)
                (`/Engine/EditorBlueprintResources/StandardMacros.IsValid` _array_element_4
                  (:`Is Valid`
                    (bind _asbpi_computer_4 (cast `/Game/Blueprints/Libraries/BPI_Computer` _array_element_4))
                    (`/Game/Blueprints/Libraries/BPI_Computer.Slot_Trigger` _asbpi_computer_4)))))
            (:`4`
              (`SceneComponent.SetVisibility` (`self.ComputerBoard4`) true false)
              (for _array_element_5 (`self.Slot4_Target`)
                (`/Engine/EditorBlueprintResources/StandardMacros.IsValid` _array_element_5
                  (:`Is Valid`
                    (bind _asbpi_computer_5 (cast `/Game/Blueprints/Libraries/BPI_Computer` _array_element_5))
                    (`/Game/Blueprints/Libraries/BPI_Computer.Slot_Trigger` _asbpi_computer_5)))))
            (:`5`
              (`SceneComponent.SetVisibility` (`self.ComputerBoard5`) true false)
              (for _array_element_6 (`self.Slot5_Target`)
                (`/Engine/EditorBlueprintResources/StandardMacros.IsValid` _array_element_6
                  (:`Is Valid`
                    (bind _asbpi_computer_6 (cast `/Game/Blueprints/Libraries/BPI_Computer` _array_element_6))
                    (`/Game/Blueprints/Libraries/BPI_Computer.Slot_Trigger` _asbpi_computer_6)))))
            (:`6`
              (`SceneComponent.SetVisibility` (`self.ComputerBoard6`) true false)
              (for _array_element_7 (`self.Slot6_Target`)
                (`/Engine/EditorBlueprintResources/StandardMacros.IsValid` _array_element_7
                  (:`Is Valid`
                    (bind _asbpi_computer_7 (cast `/Game/Blueprints/Libraries/BPI_Computer` _array_element_7))
                    (`/Game/Blueprints/Libraries/BPI_Computer.Slot_Trigger` _asbpi_computer_7)))))
            (:`7`
              (`SceneComponent.SetVisibility` (`self.ComputerBoard7`) true false)
              (for _array_element_8 (`self.Slot7_Target`)
                (`/Engine/EditorBlueprintResources/StandardMacros.IsValid` _array_element_8
                  (:`Is Valid`
                    (bind _asbpi_computer_8 (cast `/Game/Blueprints/Libraries/BPI_Computer` _array_element_8))
                    (`/Game/Blueprints/Libraries/BPI_Computer.Slot_Trigger` _asbpi_computer_8)))))))))))

(fn `UserConstructionScript`)