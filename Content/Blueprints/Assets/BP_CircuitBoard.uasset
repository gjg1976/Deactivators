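; BP_CircuitBoard is a circuit board actor that plays a fall sound when it lands.
; It records its location at BeginPlay and on every mesh hit.
; A hit plays the 2D sound only when NotPickable is false and the board is farther than a threshold distance from that recorded location, filtering out small contacts.
; SetGravity only stores a gravity force value.
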(event `self.SM_ComputerBoard.OnComponentHit`
  (params (HitComponent :type "PrimitiveComponent Object Reference") (OtherActor :type "Actor Object Reference") (OtherComp :type "PrimitiveComponent Object Reference") (NormalImpulse :type "Vector Structure") (Hit :type "HitResult Structure (by ref)"))
  (if (and (not (`self.NotPickable`)) (> (`KismetMathLibrary.Vector_Distance` (`self.AirLocation`) (`self.K2_GetActorLocation`)) (`self.Distance`)))
    (`GameplayStatics.PlaySound2D` "/Game/Sounds/fall_sound.fall_sound" 1.0 1.0 0.0 null null))
  (set `self.AirLocation` (`self.K2_GetActorLocation`)))

(event `self.ReceiveBeginPlay`
  (set `self.AirLocation` (`self.K2_GetActorLocation`)))

(fn `SetGravity`
  (params (InGravity :type "Float (double-precision)"))
  (set `self.GravityForce` InGravity))

(fn `UserConstructionScript`)