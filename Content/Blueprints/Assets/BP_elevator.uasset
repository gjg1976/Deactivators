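; Pool elevator that carries a BP_Deactivator3 or BP_Guardian up or down between its pool and top trigger boxes.
; Overlaps lock the passenger's movement and start timelines that move it along tracks rotated to the elevator's floor, ceiling or wall orientation.
; Deactivator rides can reverse mid-travel, throttled by a timer-driven keyboard lock.
; An occupied elevator nudges the other character type away; its force field kills Deactivators until SlotTrigger disables it.
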(event `self.ReceiveBeginPlay`
  (bind (_returnvalue_x _returnvalue_y _returnvalue_z) (`KismetMathLibrary.BreakVector` (`self.GetActorUpVector`)))
  (`KismetSystemLibrary.K2_SetTimerDelegate` (delegate `OnKeyboardBlock`) 0.2 true)
  (if (< _returnvalue_z -0.5)
    (set `self.LoadRotation` (struct :`Roll` 180.0))
    (if (`self.bForceField`) :!label _label
      (`ActorComponent.Activate` (`self.ForceField`) false))
    (elif (> _returnvalue_z 0.5)
      (set `self.LoadRotation` (struct))
      (goto _label)
      (elif (< _returnvalue_y -0.5)
        (set `self.LoadRotation` (struct :`Roll` -90.0))
        (if (`self.bForceField`) :!label _label_2
          (`ActorComponent.Activate` (`self.ForceFieldRot`) false))
        (elif (> _returnvalue_y 0.5)
          (set `self.LoadRotation` (struct :`Roll` 90.0))
          (goto _label_2))))))

(event `OnKeyboardBlock`
  (if (> (`self.KeyboardLock`) 0)
    (set `self.KeyboardLock` (- (`self.KeyboardLock`) 1))))

(event `self.TopBox.OnComponentBeginOverlap`
  (params (OverlappedComponent :type "PrimitiveComponent Object Reference") (OtherActor :type "Actor Object Reference") (OtherComp :type "PrimitiveComponent Object Reference") (OtherBodyIndex :type Integer) (bFromSweep :type Boolean) (SweepResult :type "HitResult Structure (by ref)"))
  (bind _triggeractor (`self.TriggerActor`))
  (bind _deactivatorpassenger (`self.DeactivatorPassenger`))
  (bind _guardianpassenger (`self.GuardianPassenger`))
  (bind _triggeractor_2 (`self.TriggerActor`))
  (bind _capsulecomponent (`Character.CapsuleComponent` (`self.GuardianPassenger`)))
  (bind _capsulecomponent_2 (`Character.CapsuleComponent` (`self.DeactivatorPassenger`)))
  (set `self.TriggerActor` OtherActor)
  (`/Engine/EditorBlueprintResources/StandardMacros.IsValid` (`self.Passenger`)
    (:`Is Valid`
      (if (not (== (`self.Passenger`) (`self.TriggerActor`)))
        (bind _asbp_deactivator_3 (cast `/Game/PortalSystem/DemoContent/ThirdPersonBP/Blueprints/BP_Deactivator3` (`self.TriggerActor`) :!label _label_3)
          (:`then`
            (`/Engine/EditorBlueprintResources/StandardMacros.IsValid` (`self.GuardianPassenger`)
              (:`Is Valid`
                (`self.K2_SetActorLocation` _triggeractor (+ (`KismetMathLibrary.MakeVector` -50.0) (`self.K2_GetActorLocation` _triggeractor)) false false))
              (:`Is Not Valid`
                (set `self.DeactivatorPassenger` _asbp_deactivator_3)
                (if (`self.bForceField`)
                  (bind _asbpi_kill (cast `/Game/Blueprints/BPI_Kill` (`self.DeactivatorPassenger`)))
                  (`/Game/Blueprints/BPI_Kill.KillActor` _asbpi_kill)
                  (set `self.DeactivatorPassenger` null)
                  (set `self.TravellingDirection` "NewEnumerator0")
                  (elif (`self.bEnabled`)
                    (set `self.Passenger` (`self.TriggerActor`))
                    (set `self.TravellingDirection` "NewEnumerator1")
                    (`CharacterMovementComponent.DisableMovement` (`Character.CharacterMovement` (`self.DeactivatorPassenger`)))
                    (set `self.KeyboardLock` 3)
                    (`self.K2_SetActorRotation` _deactivatorpassenger (`self.GetActorRotationToTravell` _deactivatorpassenger) false)
                    (`self.K2_SetActorLocation` (`self.DeactivatorPassenger`) (`SceneComponent.K2_GetComponentLocation` (`self.TopBox`)) false false)
                    (set `/Game/PortalSystem/DemoContent/ThirdPersonBP/Blueprints/BP_Deactivator3.OnPool` self (`self.DeactivatorPassenger`))
                    (set `self.PassengerInitPosition` (+ (`SceneComponent.K2_GetComponentLocation` (`self.Pool`)) (* (`SceneComponent.GetUpVector` _capsulecomponent_2) (`.OutHalfHeight` (`CapsuleComponent.GetScaledCapsuleSize` _capsulecomponent_2)) 1.1) (* (`SceneComponent.GetRightVector` _capsulecomponent_2) -10.0)))
                    (`GameplayStatics.PlaySound2D` "/Game/Sounds/pool_down.pool_down" 1.0 1.0 0.0 null null)
                    (else
                      (set `self.DeactivatorPassenger` null)
                      (set `self.TravellingDirection` "NewEnumerator0")))))))
          (:`CastFailed`
            (bind _asbp_guardian (cast `/Game/Blueprints/Assets/BP_Guardian` (`self.TriggerActor`)))
            (`/Engine/EditorBlueprintResources/StandardMacros.IsValid` (`self.DeactivatorPassenger`)
              (:`Is Valid`
                (`self.K2_SetActorLocation` _triggeractor_2 (+ (`KismetMathLibrary.MakeVector` -50.0) (`self.K2_GetActorLocation` _triggeractor_2)) false false))
              (:`Is Not Valid`
                (if (not (`self.bForceField`))
                  (set `self.GuardianPassenger` _asbp_guardian)
                  (if (`self.bEnabled`)
                    (set `self.Passenger` (`self.TriggerActor`))
                    (set `self.TravellingDirection` "NewEnumerator1")
                    (`CharacterMovementComponent.DisableMovement` (`Character.CharacterMovement` (`self.GuardianPassenger`)))
                    (`self.K2_SetActorRotation` _guardianpassenger (`self.GetActorRotationToTravell` _guardianpassenger) false)
                    (`self.K2_SetActorLocation` (`self.GuardianPassenger`) (`SceneComponent.K2_GetComponentLocation` (`self.TopBox`)) false false)
                    (set `self.PassengerInitPosition` (+ (`SceneComponent.K2_GetComponentLocation` (`self.Pool`)) (* (`SceneComponent.GetUpVector` _capsulecomponent) (`.OutHalfHeight` (`CapsuleComponent.GetScaledCapsuleSize` _capsulecomponent)) 1.1) (* (`SceneComponent.GetRightVector` _capsulecomponent) -10.0)))
                    (`GameplayStatics.PlaySound2D` "/Game/Sounds/pool_down.pool_down" 1.0 1.0 0.0 null null)
                    (else
                      (set `self.GuardianPassenger` null)
                      (set `self.TravellingDirection` "NewEnumerator0"))))))))))
    (:`Is Not Valid`
      (goto _label_3))))

(event `OnReverseDirection`
  (params (OnDirectionUp :type Boolean))
  (if (== (`self.KeyboardLock`) 0)
    (set `self.KeyboardLock` 2)
    (if OnDirectionUp
      (switch `/Game/Blueprints/Assets/E_Dea_PoolDirection` (`self.TravellingDirection`)
        (:`NewEnumerator1`
          (set `self.TravellingDirection` "NewEnumerator3"))
        (:`NewEnumerator4`
          (set `self.TravellingDirection` "NewEnumerator2")))
      (`GameplayStatics.PlaySound2D` "/Game/Sounds/pool_up.pool_up" 1.0 1.0 0.0 null null)
      (else
        (switch `/Game/Blueprints/Assets/E_Dea_PoolDirection` (`self.TravellingDirection`)
          (:`NewEnumerator2`
            (set `self.TravellingDirection` "NewEnumerator4"))
          (:`NewEnumerator3`
            (set `self.TravellingDirection` "NewEnumerator1")))
        (`GameplayStatics.PlaySound2D` "/Game/Sounds/pool_down.pool_down" 1.0 1.0 0.0 null null)))
    (switch `/Game/Blueprints/Assets/E_Dea_PoolDirection` (`self.TravellingDirection`) :!label _label_4
      (:`NewEnumerator1`
        (bind (_direction _deactivatortrackup) (`Timeline|TimelineDown` :`NewTime` 0.2 :!label _label_5)
          (:`Update`
            (`self.K2_SetActorLocation` (`self.Passenger`) (+ (`KismetMathLibrary.GreaterGreater_VectorRotator` _deactivatortrackup (`self.LoadRotation`)) (`self.PassengerInitPosition`)) false false))
          (:`Finished`
            (`CharacterMovementComponent.SetMovementMode` (`Character.CharacterMovement` (`self.DeactivatorPassenger`)) "MOVE_Walking" 0 :!label _label_6)
            (set `self.TravellingDirection` "NewEnumerator0")
            (set `/Game/PortalSystem/DemoContent/ThirdPersonBP/Blueprints/BP_Deactivator3.OnPool` null (`self.DeactivatorPassenger`))
            (set `self.Passenger` null)
            (set `self.DeactivatorPassenger` null)
            (bind _outactors (`GameplayStatics.GetAllActorsOfClass` "/Game/Blueprints/Building/BP_BuildingGenerator.BP_BuildingGenerator_C"))
            (if (> (`KismetArrayLibrary.Array_Length` _outactors) 0)
              (`/Game/Blueprints/Building/BP_BuildingGenerator.SetKeyboardEnable` (`|GetArrayItem` _outactors) true)))))
      (:`NewEnumerator2`
        (bind (_direction_2 _deactivatortrackup_2) (`Timeline|TimelineUp` :`NewTime` 0.2 :!label _label_7)
          (:`Update`
            (`self.K2_SetActorLocation` (`self.Passenger`) (+ (`KismetMathLibrary.GreaterGreater_VectorRotator` _deactivatortrackup_2 (`self.LoadRotation`)) (`self.PassengerInitPosition`)) false false))
          (:`Finished`
            (goto _label_6))))
      (:`NewEnumerator3`
        (goto _label_5 :!via `Reverse`))
      (:`NewEnumerator4`
        (goto _label_7 :!via `Reverse`)))))

(event `self.PoolBox.OnComponentBeginOverlap`
  (params (OverlappedComponent :type "PrimitiveComponent Object Reference") (OtherActor :type "Actor Object Reference") (OtherComp :type "PrimitiveComponent Object Reference") (OtherBodyIndex :type Integer) (bFromSweep :type Boolean) (SweepResult :type "HitResult Structure (by ref)"))
  (bind _guardianpassenger (`self.GuardianPassenger`))
  (bind _triggeractor (`self.TriggerActor`))
  (bind _triggeractor_2 (`self.TriggerActor`))
  (bind _deactivatorpassenger (`self.DeactivatorPassenger`))
  (bind _capsulecomponent (`Character.CapsuleComponent` (`self.GuardianPassenger`)))
  (bind _capsulecomponent_2 (`Character.CapsuleComponent` (`self.DeactivatorPassenger`)))
  (set `self.TriggerActor` OtherActor)
  (if (`self.bEnabled`)
    (bind _asbp_deactivator_3 (cast `/Game/PortalSystem/DemoContent/ThirdPersonBP/Blueprints/BP_Deactivator3` (`self.TriggerActor`))
      (:`then`
        (`/Engine/EditorBlueprintResources/StandardMacros.IsValid` (`self.GuardianPassenger`)
          (:`Is Valid`
            (`self.K2_SetActorLocation` _triggeractor (+ (`KismetMathLibrary.MakeVector` -50.0) (`self.K2_GetActorLocation` _triggeractor)) false false))
          (:`Is Not Valid`
            (set `self.DeactivatorPassenger` _asbp_deactivator_3)
            (if (`self.bForceField`)
              (bind _asbpi_kill (cast `/Game/Blueprints/BPI_Kill` (`self.DeactivatorPassenger`)))
              (`/Game/Blueprints/BPI_Kill.KillActor` _asbpi_kill)
              (set `self.DeactivatorPassenger` null)
              (else
                (bind _outactors (`GameplayStatics.GetAllActorsOfClass` "/Game/Blueprints/Building/BP_BuildingGenerator.BP_BuildingGenerator_C"))
                (if (> (`KismetArrayLibrary.Array_Length` _outactors) 0)
                  (`/Game/Blueprints/Building/BP_BuildingGenerator.SetKeyboardEnable` (`|GetArrayItem` _outactors) false)
                  (`/Engine/EditorBlueprintResources/StandardMacros.IsValid` (`self.Passenger`)
                    (:`Is Valid`
                      (if (== (`self.Passenger`) (`self.TriggerActor`))
                        (`|ExecutionSequence`
                          (:`then_0`
                            (goto _label_5 :!via `SetNewTime`))
                          (:`then_1`
                            (goto _label_4)))))
                    (:`Is Not Valid`
                      (`CharacterMovementComponent.DisableMovement` (`Character.CharacterMovement` (`self.DeactivatorPassenger`)))
                      (set `self.Passenger` (`self.TriggerActor`))
                      (`self.K2_SetActorRotation` _deactivatorpassenger (`self.GetActorRotationToTravell` _deactivatorpassenger) false)
                      (set `self.KeyboardLock` 2)
                      (set `/Game/PortalSystem/DemoContent/ThirdPersonBP/Blueprints/BP_Deactivator3.OnPool` self (`self.DeactivatorPassenger`))
                      (set `self.PassengerInitPosition` (+ (`SceneComponent.K2_GetComponentLocation` (`self.Pool`)) (* (`SceneComponent.GetUpVector` _capsulecomponent_2) (`.OutHalfHeight` (`CapsuleComponent.GetScaledCapsuleSize` _capsulecomponent_2))) (* (`SceneComponent.GetRightVector` _capsulecomponent_2) -10.0)))
                      (set `self.TravellingDirection` "NewEnumerator2")
                      (`GameplayStatics.PlaySound2D` "/Game/Sounds/pool_up.pool_up" 1.0 1.0 0.0 null null)
                      (`|ExecutionSequence`
                        (:`then_0`
                          (goto _label_7 :!via `SetNewTime`))
                        (:`then_1`
                          (goto _label_4)))))))))))
      (:`CastFailed`
        (bind _asbp_guardian (cast `/Game/Blueprints/Assets/BP_Guardian` (`self.TriggerActor`)))
        (`/Engine/EditorBlueprintResources/StandardMacros.IsValid` (`self.DeactivatorPassenger`)
          (:`Is Valid`
            (`self.K2_SetActorLocation` _triggeractor_2 (+ (`KismetMathLibrary.MakeVector` -50.0) (`self.K2_GetActorLocation` _triggeractor_2)) false false))
          (:`Is Not Valid`
            (if (not (`self.bForceField`))
              (set `self.GuardianPassenger` _asbp_guardian)
              (`/Engine/EditorBlueprintResources/StandardMacros.IsValid` (`self.Passenger`)
                (:`Is Valid`
                  (if (== (`self.Passenger`) (`self.TriggerActor`))
                    (`|ExecutionSequence`
                      (:`then_0`
                        (bind (_direction _deactivatortrackup) (`Timeline|Timeline_0` :`NewTime` 0.2 :!via `SetNewTime` :!label _label_8)
                          (:`Update`
                            (`self.K2_SetActorLocation` (`self.Passenger`) (+ (`KismetMathLibrary.GreaterGreater_VectorRotator` _deactivatortrackup (`self.LoadRotation`)) (`self.PassengerInitPosition`)) false false))
                          (:`Finished`
                            (`CharacterMovementComponent.SetMovementMode` (`Character.CharacterMovement` (`self.GuardianPassenger`)) "MOVE_Walking" 0)
                            (set `self.TravellingDirection` "NewEnumerator0")
                            (set `self.Passenger` null)
                            (set `self.GuardianPassenger` null))))
                      (:`then_1`
                        (switch `/Game/Blueprints/Assets/E_Dea_PoolDirection` (`self.TravellingDirection`) :!label _label_9
                          (:`NewEnumerator1`
                            (goto _label_8))
                          (:`NewEnumerator2`
                            (bind (_direction_2 _deactivatortrackup_2) (`Timeline|Timeline` :`NewTime` 0.2 :!label _label_10)
                              (:`Update`
                                (`self.K2_SetActorLocation` (`self.Passenger`) (+ (`KismetMathLibrary.GreaterGreater_VectorRotator` _deactivatortrackup_2 (`self.LoadRotation`)) (`self.PassengerInitPosition`)) false false))
                              (:`Finished`
                                (`CharacterMovementComponent.SetMovementMode` (`Character.CharacterMovement` (`self.GuardianPassenger`)) "MOVE_Walking" 0)
                                (set `self.TravellingDirection` "NewEnumerator0")
                                (set `self.Passenger` null)
                                (set `self.GuardianPassenger` null)))))))))
                (:`Is Not Valid`
                  (`CharacterMovementComponent.DisableMovement` (`Character.CharacterMovement` (`self.GuardianPassenger`)))
                  (set `self.Passenger` (`self.TriggerActor`))
                  (`self.K2_SetActorRotation` _guardianpassenger (`self.GetActorRotationToTravell` _guardianpassenger) false)
                  (set `self.PassengerInitPosition` (+ (`SceneComponent.K2_GetComponentLocation` (`self.Pool`)) (* (`SceneComponent.GetUpVector` _capsulecomponent) (`.OutHalfHeight` (`CapsuleComponent.GetScaledCapsuleSize` _capsulecomponent))) (* (`SceneComponent.GetRightVector` _capsulecomponent) -10.0)))
                  (set `self.TravellingDirection` "NewEnumerator2")
                  (`GameplayStatics.PlaySound2D` "/Game/Sounds/pool_up.pool_up" 1.0 1.0 0.0 null null)
                  (`|ExecutionSequence`
                    (:`then_0`
                      (goto _label_10 :!via `SetNewTime`))
                    (:`then_1`
                      (goto _label_9))))))))))))

(event `/Game/Blueprints/Libraries/BPI_Computer.Slot_Trigger`
  (set `self.bForceField` false)
  (`ActorComponent.Deactivate` (`self.ForceField`))
  (`ActorComponent.Deactivate` (`self.ForceFieldRot`)))

(fn `GetActorRotationToTravell`
  (params (InActor :type "Actor Object Reference"))
  (returns (OutRotator :type "Rotator Structure"))
  (bind (_returnvalue_x _returnvalue_y _returnvalue_z) (`KismetMathLibrary.BreakVector` (`self.GetActorUpVector` InActor)))
  (if (< _returnvalue_z -0.5)
    (return (struct :`Pitch` 180.0))
    (elif (> _returnvalue_z 0.5)
      (return (struct :`Yaw` 180.0))
      (elif (< _returnvalue_y -0.5)
        (return (struct :`Pitch` 180.0 :`Roll` -90.0))
        (elif (> _returnvalue_y 0.5)
          (return (struct :`Pitch` 180.0 :`Roll` 90.0))
          (else
            (return)))))))

(fn `Kill Player`
  (bind _outactors (`GameplayStatics.GetAllActorsOfClass` null))
  (`/Engine/EditorBlueprintResources/StandardMacros.CompareInt` (`KismetArrayLibrary.Array_Length` _outactors)))

(fn `UserConstructionScript`)