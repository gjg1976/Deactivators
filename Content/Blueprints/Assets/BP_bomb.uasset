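; BP_bomb is a bomb actor with a timed fuse that blows up rooms of the generated building.
; A one-second timer ignites it and later detonates it, with fuse times and bounce limit divided by the game mode multiplier.
; Pickable bombs also explode when hits after sufficient travel exhaust their bounces.
; Blowing detaches it from any deactivator, damages its room, shakes cameras and has BP_BuildingGenerator check remaining bombs.
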(event `self.ReceiveBeginPlay`
  (bind _asmy_game_instance (cast `/Game/MyGameInstance` (`GameplayStatics.GetGameInstance`)))
  (bind _output_get (set `self.Multiplier` (`/Game/MyGameInstance.ModeMultiplier` _asmy_game_instance)))
  (set `self.MaxBounces` (`KismetMathLibrary.FTrunc` (/ (`self.MaxBounces`) _output_get)))
  (`KismetSystemLibrary.K2_SetTimerDelegate` (delegate `CheckBomb`) 1.0 true)
  (set `self.AirLocation` (`self.K2_GetActorLocation`))
  (if (< (`self.StartTime`) 0)
    (set `self.StartTime` 0.0))
  (if (>= (`self.StartTime`) (`self.BlowTime`))
    (set `self.BlowTime` (+ (`self.StartTime`) 1))))

(event `CheckBomb`
  (if (== (`self.TimerCount`) (/ (`self.StartTime`) (`self.Multiplier`)))
    (`GameplayStatics.PlaySound2D` "/Game/Sounds/bomb_ignited.bomb_ignited" 1.0 1.0 0.0 null null)
    (set `self.activated?` true)
    (`ActorComponent.Activate` (`self.Flame`) false)
    (set `self.TimerCount` (+ (`self.TimerCount`) 1) :!label _label)
    (elif (< (`self.TimerCount`) (/ (`self.BlowTime`) (`self.Multiplier`)))
      (goto _label)
      (else
        (`self.Blow`)))))

(event `self.SM_Bomb.OnComponentHit`
  (params (HitComponent :type "PrimitiveComponent Object Reference") (OtherActor :type "Actor Object Reference") (OtherComp :type "PrimitiveComponent Object Reference") (NormalImpulse :type "Vector Structure") (Hit :type "HitResult Structure (by ref)"))
  (if (and (not (`self.NotPickable`)) (> (`KismetMathLibrary.Vector_Distance` (`self.AirLocation`) (`self.K2_GetActorLocation`)) (`self.Distance`)))
    (if (> (`self.MaxBounces`) 0)
      (set `self.MaxBounces` (- (`self.MaxBounces`) 1))
      (`GameplayStatics.PlaySound2D` "/Game/Sounds/fall_sound.fall_sound" 1.0 1.0 0.0 null null)
      (set `self.AirLocation` (`self.K2_GetActorLocation`) :!label _label_2)
      (else
        (`self.Blow`)))
    (else
      (goto _label_2))))

(fn `Blow`
  (`GameplayStatics.PlaySound2D` "/Game/Sounds/explosion.explosion" 1.0 1.0 0.0 null null)
  (bind _asbp_deactivator_3 (cast `/Game/PortalSystem/DemoContent/ThirdPersonBP/Blueprints/BP_Deactivator3` (`self.GetAttachParentActor`))
    (:`then`
      (`/Game/PortalSystem/DemoContent/ThirdPersonBP/Blueprints/BP_Deactivator3.DetachBomb` _asbp_deactivator_3))
    (:`CastFailed`
      _))
  (bind _returnvalue (`GameplayStatics.GetActorOfClass` "/Game/Blueprints/Building/BP_BuildingGenerator.BP_BuildingGenerator_C"))
  (`/Engine/EditorBlueprintResources/StandardMacros.IsValid` _returnvalue
    (:`Is Valid`
      (bind _outroom (`/Game/Blueprints/Building/BP_BuildingGenerator.GetRoomByLocation` _returnvalue (`self.K2_GetActorLocation`)))
      (`/Engine/EditorBlueprintResources/StandardMacros.IsValid` _outroom
        (:`Is Valid`
          (`/Game/Blueprints/Building/Room/BP_RoomGenerator.Blows` _outroom))
        (:`Is Not Valid`
          _))
      (`/Game/Blueprints/Building/BP_BuildingGenerator.OnCamerasShake` _returnvalue)
      (`self.K2_DestroyActor`)
      (`/Game/Blueprints/Building/BP_BuildingGenerator.OnCheckBombs` _returnvalue))))

(fn `GetTimePorcent`
  (returns (TimePorcent :type "Float (double-precision)") (Activated :type Boolean))
  (bind _starttime (`self.StartTime`))
  (bind _activated_ (`self.activated?`))
  (bind _returnvalue (- (`self.BlowTime`) _starttime))
  (if _activated_
    (set `self.ReturnPorcent` (/ (- _returnvalue (- (`self.TimerCount`) _starttime)) _returnvalue))
    (else
      (set `self.ReturnPorcent` 1.0)))
  (return (`self.ReturnPorcent`) _activated_))

(fn `SetGravity`
  (params (InGravity :type "Float (double-precision)"))
  (set `self.GravityForce` InGravity))

(fn `UserConstructionScript`)