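; BP_DoorForceField is a door force field that blocks a set of tiles until it is triggered.
; On BeginPlay it sets ForceNoWalkable on every valid entry in Tiles.
; The SlotTrigger event clears that flag on the same tiles, then destroys the actor.
; Any BP_Deactivator3 that begins overlapping the ForceField component is killed through its KillActor call.
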(event `self.ReceiveBeginPlay`
  (for _array_element (`self.Tiles`)
    (`/Engine/EditorBlueprintResources/StandardMacros.IsValid` _array_element
      (:`Is Valid`
        (set `/Game/Blueprints/Building/Tiles/BP_Tile.bForceNoWalkable` true _array_element)))))

(event `/Game/Blueprints/Libraries/BPI_Computer.Slot_Trigger`
  (for _array_element (`self.Tiles`)
    (`/Engine/EditorBlueprintResources/StandardMacros.IsValid` _array_element
      (:`Is Valid`
        (set `/Game/Blueprints/Building/Tiles/BP_Tile.bForceNoWalkable` false _array_element))))
  (`self.K2_DestroyActor`))

(event `self.ForceField.OnComponentBeginOverlap`
  (params (OverlappedComponent :type "PrimitiveComponent Object Reference") (OtherActor :type "Actor Object Reference") (OtherComp :type "PrimitiveComponent Object Reference") (OtherBodyIndex :type Integer) (bFromSweep :type Boolean) (SweepResult :type "HitResult Structure (by ref)"))
  (bind _asbp_deactivator_3 (cast `/Game/PortalSystem/DemoContent/ThirdPersonBP/Blueprints/BP_Deactivator3` OtherActor))
  (`/Game/PortalSystem/DemoContent/ThirdPersonBP/Blueprints/BP_Deactivator3.KillActor` _asbp_deactivator_3))

(fn `UserConstructionScript`)