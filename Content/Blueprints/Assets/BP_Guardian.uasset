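; Guardian AI character that patrols random nav-grid tiles and chases BP_Deactivator3 instigators it hears.
; BP_NavGridGenerator supplies paths, which Tick follows with orientation-aware steering for floors, walls and ceilings.
; When several guardians target the same deactivator, distance arbitration picks the closer one, and a looping timer resumes patrol pathing once hearing lapses.
; Each landing costs a hit that auto-repairs over time; running out awards score and destroys the guardian.
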(event `self.ReceiveBeginPlay`
  (bind _asmy_game_instance (cast `/Game/MyGameInstance` (`GameplayStatics.GetGameInstance`)))
  (set `self.Multiplier` (`/Game/MyGameInstance.ModeMultiplier` _asmy_game_instance))
  (`KismetSystemLibrary.K2_SetTimerDelegate` (delegate `CheckPatrolling`) 0.6 true)
  (`self.SetStartTile`)
  (bind _asbp_nav_grid_generator (cast `/Game/Blueprints/Building/BP_NavGridGenerator` (`self.GetOwner` (`self.GetOwner` (`self.HitStarTile`)))))
  (`self.SetPatrollingPath` _asbp_nav_grid_generator))

(event `CheckPatrolling`
  (if (== (`self.AutorepairCounter`) 0)
    (set `self.HitCounts` 2)
    (else
      (set `self.AutorepairCounter` (- (`self.AutorepairCounter`) 1))))
  (if (`self.bHearing`)
    (set `self.bHearing` false)
    (else
      (set `self.chasingTarget` null)
      (bind _asbp_nav_grid_generator (cast `/Game/Blueprints/Building/BP_NavGridGenerator` (`self.GetOwner` (`self.GetOwner` (`self.HitStarTile`)))))
      (if (not (> (`self.NextPatrollingIndex`) 0))
        (bind _asbp_nav_grid (cast `/Game/Blueprints/Building/Grid/BP_NavGrid` (`self.GetOwner` (`self.HitStarTile`))))
        (bind _outrandomtile (`/Game/Blueprints/Building/Grid/BP_NavGrid.GetRandomWalkingTileTile` _asbp_nav_grid))
        (set `self.HitEndTile` _outrandomtile)
        (`/Game/Blueprints/Building/BP_NavGridGenerator.NavGridFindPathTo` _asbp_nav_grid_generator (`self.HitStarTile`) (`self.HitEndTile`) self)))))

(event `/Game/Blueprints/Libraries/BPI_search.OnSetPath`
  (params (InPath :type "Array of /Game/Blueprints/Building/Tiles/BP_Tile Object Reference (by ref)"))
  (bind _returnvalue (`KismetArrayLibrary.Array_Length` (`self.ActivePath`)))
  (bind _returnvalue_2 (`KismetArrayLibrary.Array_Length` (`self.PatrollingPath`)))
  (bind _returnvalue_3 (- _returnvalue_2 2))
  (bind _returnvalue_4 (- _returnvalue 2))
  (if (`self.bPatrolling`)
    (bind _output_get (set `self.PatrollingPath` InPath))
    (if (> _returnvalue_2 1)
      (set `self.NextPatrollingTile` (`|GetArrayItem` _output_get _returnvalue_3))
      (set `self.NextPatrollingIndex` _returnvalue_3))
    (else
      (bind _output_get_2 (set `self.ActivePath` InPath))
      (if (> _returnvalue 1)
        (set `self.NextTile` (`|GetArrayItem` _output_get_2 _returnvalue_4))
        (set `self.NextIndex` _returnvalue_4)))))

(event `self.ReceiveTick`
  (params (DeltaSeconds :type "Float (single-precision)"))
  (bind (_outrotation _bstop) (`self.GetMovementStatus`))
  (bind (_outrotation_2 _bstop_2) (`self.GetPatrollingMovementStatus`))
  (bind _nexttile (`self.NextTile`))
  (bind _nextpatrollingtile (`self.NextPatrollingTile`))
  (bind _returnvalue (- (`self.NextPatrollingIndex`) 1))
  (bind _returnvalue_2 (- (`self.NextIndex`) 1))
  (`|ExecutionSequence`
    (:`then_0`
      (if (`self.bPatrolling`)
        ; Chasing
        (`|ExecutionSequence`
          (:`then_0`
            (`self.SetStartTile`))
          (:`then_1`
            (`/Engine/EditorBlueprintResources/StandardMacros.IsValid` _nextpatrollingtile
              (:`Is Valid`
                (if _bstop_2
                  (if (> (`self.NextPatrollingIndex`) 0)
                    (set `self.NextPatrollingTile` (`|GetArrayItem` (`self.PatrollingPath`) _returnvalue))
                    (set `self.NextPatrollingIndex` _returnvalue)
                    (else
                      (`self.ClearPatrollingPath`)))
                  (else
                    (`self.AddMovementInput` (/ (`KismetMathLibrary.Normal` (- (`self.K2_GetActorLocation` _nextpatrollingtile) (`self.K2_GetActorLocation`))) (/ (`self.Multiplier`) (`CharacterMovementComponent.MaxWalkSpeed` (`self.CharacterMovement`)))))
                    (`self.K2_SetActorRotation` (`KismetMathLibrary.Quat_Rotator` (`KismetMathLibrary.Quat_Slerp` (`KismetMathLibrary.Conv_RotatorToQuaternion` (`self.K2_GetActorRotation`)) (`KismetMathLibrary.Conv_RotatorToQuaternion` _outrotation_2) (`KismetMathLibrary.FClamp` (* DeltaSeconds 5.0)))))))))))
        (else
          ; Chasing
          (`|ExecutionSequence`
            (:`then_0`
              (`self.SetStartTile`))
            (:`then_1`
              (`/Engine/EditorBlueprintResources/StandardMacros.IsValid` _nexttile
                (:`Is Valid`
                  (if _bstop
                    (if (> (`self.NextIndex`) 0)
                      (set `self.NextTile` (`|GetArrayItem` (`self.ActivePath`) _returnvalue_2))
                      (set `self.NextIndex` _returnvalue_2)
                      (else
                        (`self.ClearPath`)))
                    (else
                      (`self.AddMovementInput` (/ (`KismetMathLibrary.Normal` (- (`self.K2_GetActorLocation` _nexttile) (`self.K2_GetActorLocation`))) (/ 1.0 (`CharacterMovementComponent.MaxWalkSpeed` (`self.CharacterMovement`)))))
                      (`self.K2_SetActorRotation` (`KismetMathLibrary.Quat_Rotator` (`KismetMathLibrary.Quat_Slerp` (`KismetMathLibrary.Conv_RotatorToQuaternion` (`self.K2_GetActorRotation`)) (`KismetMathLibrary.Conv_RotatorToQuaternion` _outrotation) (`KismetMathLibrary.FClamp` (* DeltaSeconds 5.0))))))))))))))
    (:`then_1`
      (if (and (`self.InAir?`) (not (`NavMovementComponent.IsFalling` (`self.CharacterMovement`))))
        (`GameplayStatics.PlaySound2D` "/Game/Sounds/fall_sound.fall_sound" 1.0 1.0 0.0 null null)
        (set `self.InAir?` false)
        (bind _output_get (set `self.HitCounts` (- (`self.HitCounts`) 1)))
        (set `self.AutorepairCounter` 20)
        (if (<= _output_get 0)
          (`CharacterMovementComponent.DisableMovement` (`self.CharacterMovement`))
          (`ActorComponent.Activate` (`self.NS_Basic_3`) false)
          (`ActorComponent.Activate` (`self.NS_Fire_Floor_01_Smoke`) false)
          (`GameplayStatics.PlaySound2D` "/Game/Sounds/deintegration.deintegration" 1.0 1.0 0.0 null null)
          (bind _returnvalue_3 (`GameplayStatics.GetActorOfClass` "/Game/Blueprints/Building/BP_BuildingGenerator.BP_BuildingGenerator_C"))
          (`/Engine/EditorBlueprintResources/StandardMacros.IsValid` _returnvalue_3
            (:`Is Valid`
              (`/Game/Blueprints/Building/BP_BuildingGenerator.AddScore` _returnvalue_3 "NewEnumerator2" null))
            (:`Is Not Valid`
              _))
          (`KismetSystemLibrary.Delay` 1.5)
          (`self.K2_DestroyActor`))
        (elif (and (not (`self.InAir?`)) (`NavMovementComponent.IsFalling` (`self.CharacterMovement`)))
          (set `self.InAir?` true))))))

(event `self.PawnSensing.OnHearNoise`
  (params (Instigator :type "Pawn Object Reference") (Location :type "Vector Structure (by ref)") (Volume :type "Float (single-precision)"))
  (set `self.bHearing` true)
  (bind _asbp_deactivator_3 (cast `/Game/PortalSystem/DemoContent/ThirdPersonBP/Blueprints/BP_Deactivator3` Instigator))
  (`self.ClearPath`)
  (`self.SetStartTile`)
  (`self.SetEndTile` _asbp_deactivator_3)
  (`/Engine/EditorBlueprintResources/StandardMacros.IsValid` (`self.HitStarTile`)
    (:`Is Valid`
      (`/Engine/EditorBlueprintResources/StandardMacros.IsValid` (`self.HitEndTile`)
        (:`Is Valid`
          (bind _asbp_nav_grid_generator (cast `/Game/Blueprints/Building/BP_NavGridGenerator` (`self.GetOwner` (`self.GetOwner` (`self.HitStarTile`)))))
          (set `self.bPatrolling` false)
          (`/Game/Blueprints/Building/BP_NavGridGenerator.NavGridFindPathTo` _asbp_nav_grid_generator (`self.HitStarTile`) (`self.HitEndTile`) self)
          (if (== (`KismetArrayLibrary.Array_Length` (`self.ActivePath`)) 0)
            (if (< (`KismetArrayLibrary.Array_Length` (`self.PatrollingPath`)) 2) :!label _label
              (`self.SetPatrollingPath` _asbp_nav_grid_generator)
              (else
                (set `self.bPatrolling` true)))
            (set `self.chasingTarget` null)
            (else
              (bind _outsucess (`self.CheckChasingTarget` _asbp_deactivator_3))
              (if _outsucess
                (`self.ClearPatrollingPath`)
                (set `self.chasingTarget` _asbp_deactivator_3)
                (else
                  (goto _label))))))))))

(event `OnDeintegrateDeactivator`
  (params (InDeactivator :type "/Game/PortalSystem/DemoContent/ThirdPersonBP/Blueprints/BP_Deactivator3 Object Reference"))
  (`ActorComponent.Activate` (`self.SparkRight`) false)
  (`ActorComponent.Activate` (`self.SparkLeft`) false)
  (`KismetSystemLibrary.Delay` 1.5)
  (`ActorComponent.Deactivate` (`self.SparkRight`))
  (`ActorComponent.Deactivate` (`self.SparkLeft`)))

(fn `CheckChasingTarget`
  (params (InTarget :type "/Game/PortalSystem/DemoContent/ThirdPersonBP/Blueprints/BP_Deactivator3 Object Reference"))
  (returns (OutSucess :type Boolean))
  (bind _outactors (`GameplayStatics.GetAllActorsOfClass` "BP_Guardian_C"))
  (for _array_element _outactors
    (if (!= _array_element self)
      (if (== (`/Game/Blueprints/Assets/BP_Guardian.chasingTarget` _array_element) (`local.InTarget`))
        (if (< (`KismetMathLibrary.Vector_Distance` (`self.K2_GetActorLocation` self) (`self.K2_GetActorLocation` (`local.InTarget`))) (`KismetMathLibrary.Vector_Distance` (`self.K2_GetActorLocation` _array_element) (`self.K2_GetActorLocation` (`local.InTarget`))))
          (set `/Game/Blueprints/Assets/BP_Guardian.chasingTarget` null _array_element)
          (return true)
          (else
            (return false))))))
  (return true))

(fn `ClearPath`
  (for _array_element (`self.ActivePath`)
    (`/Engine/EditorBlueprintResources/StandardMacros.IsValid` _array_element
      (:`Is Valid`
        (message `/Game/Blueprints/Libraries/BPI_interactable.OnInteract` _array_element "NewEnumerator0"))))
  (`KismetArrayLibrary.Array_Clear` (`self.ActivePath`))
  (set `self.NextIndex` 0)
  (set `self.NextTile` null))

(fn `ClearPatrollingPath`
  (for _array_element (`self.PatrollingPath`)
    (`/Engine/EditorBlueprintResources/StandardMacros.IsValid` _array_element
      (:`Is Valid`
        (message `/Game/Blueprints/Libraries/BPI_interactable.OnInteract` _array_element "NewEnumerator0"))))
  (`KismetArrayLibrary.Array_Clear` (`self.PatrollingPath`))
  (set `self.NextPatrollingIndex` 0)
  (set `self.NextPatrollingTile` null))

(fn `GetMovementStatus`
  (returns (OutRotation :type "Rotator Structure") (bStop :type Boolean))
  (locals (LocalRotation :type "Rotator Structure" :default (struct)))
  (bind _returnvalue (`self.K2_GetActorLocation`))
  (bind _returnvalue_2 (`self.K2_GetActorLocation`))
  (bind _returnvalue_3 (`self.K2_GetActorLocation`))
  (bind _returnvalue_4 (`self.K2_GetActorLocation`))
  (bind _returnvalue_5 (`self.K2_GetActorLocation` (`self.NextTile`)))
  (bind _returnvalue_6 (`self.K2_GetActorLocation` (`self.NextTile`)))
  (bind _returnvalue_7 (`self.K2_GetActorLocation` (`self.NextTile`)))
  (bind _returnvalue_8 (`self.K2_GetActorLocation` (`self.NextTile`)))
  (`/Engine/EditorBlueprintResources/StandardMacros.IsValid` (`self.NextTile`)
    (:`Is Valid`
      (switch `/Game/Blueprints/Building/Room/E_Dea_RoomDirection` (`self.GetOrientation`)
        (:`NewEnumerator0`
          (if (> (`KismetMathLibrary.Vector_Distance` (`KismetMathLibrary.MakeVector` (.x _returnvalue_7) (.y _returnvalue_7)) (`KismetMathLibrary.MakeVector` (.x _returnvalue_3) (.y _returnvalue_3))) (`self.DistanceTolerance`))
            (set `local.LocalRotation` (`KismetMathLibrary.MakeRotator` 0.0 0.0 (`KismetMathLibrary.DegAtan2` (.y (`KismetMathLibrary.Normal` (- _returnvalue_7 _returnvalue_3))) (.x (`KismetMathLibrary.Normal` (- _returnvalue_7 _returnvalue_3))))))
            (else
              (return (struct) true))))
        (:`NewEnumerator1`
          (if (> (`KismetMathLibrary.Vector_Distance` (`KismetMathLibrary.MakeVector` (.x _returnvalue_8) 0.0 (.z _returnvalue_8)) (`KismetMathLibrary.MakeVector` (.x _returnvalue_4) 0.0 (.z _returnvalue_4))) (`self.DistanceTolerance`))
            (set `local.LocalRotation` (`KismetMathLibrary.MakeRotator` 90.0 (`KismetMathLibrary.DegAtan2` (.z (`KismetMathLibrary.Normal` (- _returnvalue_8 _returnvalue_4))) (.x (`KismetMathLibrary.Normal` (- _returnvalue_8 _returnvalue_4))))))
            (else
              (return (struct) true))))
        (:`NewEnumerator2`
          (if (> (`KismetMathLibrary.Vector_Distance` (`KismetMathLibrary.MakeVector` (.x _returnvalue_6) (.y _returnvalue_6)) (`KismetMathLibrary.MakeVector` (.x _returnvalue_2) (.y _returnvalue_2))) (`self.DistanceTolerance`))
            (set `local.LocalRotation` (`KismetMathLibrary.MakeRotator` 180.0 0.0 (`KismetMathLibrary.DegAtan2` (* (.z (`KismetMathLibrary.Normal` (- _returnvalue_6 _returnvalue_2))) -1.0) (.x (`KismetMathLibrary.Normal` (- _returnvalue_6 _returnvalue_2))))))
            (else
              (return (struct) true))))
        (:`NewEnumerator3`
          (if (> (`KismetMathLibrary.Vector_Distance` (`KismetMathLibrary.MakeVector` (.x _returnvalue_5) 0.0 (.z _returnvalue_5)) (`KismetMathLibrary.MakeVector` (.x _returnvalue) 0.0 (.z _returnvalue))) (`self.DistanceTolerance`))
            (set `local.LocalRotation` (`KismetMathLibrary.MakeRotator` -90.0 (`KismetMathLibrary.DegAtan2` (* (.z (`KismetMathLibrary.Normal` (- _returnvalue_5 _returnvalue))) -1.0) (.x (`KismetMathLibrary.Normal` (- _returnvalue_5 _returnvalue))))))
            (else
              (return (struct) true)))))
      (return (`local.LocalRotation`) false))))

(fn `GetOrientation`
  (returns (OutOrientation :type "/Game/Blueprints/Building/Room/E_Dea_RoomDirection Enum"))
  (bind _y (.y (`self.GetActorUpVector`)))
  (bind _z (.z (`self.GetActorUpVector`)))
  (if (> _y 0.5)
    (return "NewEnumerator1")
    (elif (< _y -0.5)
      (return "NewEnumerator3")
      (elif (> _z 0.5)
        (return "NewEnumerator0")
        (elif (< _z -0.5)
          (return "NewEnumerator2")
          (else
            (return "NewEnumerator0")))))))

(fn `GetPatrollingMovementStatus`
  (returns (OutRotation :type "Rotator Structure") (bStop :type Boolean))
  (locals (LocalRotation :type "Rotator Structure" :default (struct)))
  (bind _returnvalue (`self.K2_GetActorLocation`))
  (bind _returnvalue_2 (`self.K2_GetActorLocation`))
  (bind _returnvalue_3 (`self.K2_GetActorLocation`))
  (bind _returnvalue_4 (`self.K2_GetActorLocation`))
  (bind _returnvalue_5 (`self.K2_GetActorLocation` (`self.NextPatrollingTile`)))
  (bind _returnvalue_6 (`self.K2_GetActorLocation` (`self.NextPatrollingTile`)))
  (bind _returnvalue_7 (`self.K2_GetActorLocation` (`self.NextPatrollingTile`)))
  (bind _returnvalue_8 (`self.K2_GetActorLocation` (`self.NextPatrollingTile`)))
  (`/Engine/EditorBlueprintResources/StandardMacros.IsValid` (`self.NextPatrollingTile`)
    (:`Is Valid`
      (switch `/Game/Blueprints/Building/Room/E_Dea_RoomDirection` (`self.GetOrientation`)
        (:`NewEnumerator0`
          (if (> (`KismetMathLibrary.Vector_Distance` (`KismetMathLibrary.MakeVector` (.x _returnvalue_7) (.y _returnvalue_7)) (`KismetMathLibrary.MakeVector` (.x _returnvalue_3) (.y _returnvalue_3))) (`self.DistanceTolerance`))
            (set `local.LocalRotation` (`KismetMathLibrary.MakeRotator` 0.0 0.0 (`KismetMathLibrary.DegAtan2` (.y (`KismetMathLibrary.Normal` (- _returnvalue_7 _returnvalue_3))) (.x (`KismetMathLibrary.Normal` (- _returnvalue_7 _returnvalue_3))))))
            (else
              (return (struct) true))))
        (:`NewEnumerator1`
          (if (> (`KismetMathLibrary.Vector_Distance` (`KismetMathLibrary.MakeVector` (.x _returnvalue_8) 0.0 (.z _returnvalue_8)) (`KismetMathLibrary.MakeVector` (.x _returnvalue_4) 0.0 (.z _returnvalue_4))) (`self.DistanceTolerance`))
            (set `local.LocalRotation` (`KismetMathLibrary.MakeRotator` 90.0 (`KismetMathLibrary.DegAtan2` (.z (`KismetMathLibrary.Normal` (- _returnvalue_8 _returnvalue_4))) (.x (`KismetMathLibrary.Normal` (- _returnvalue_8 _returnvalue_4))))))
            (else
              (return (struct) true))))
        (:`NewEnumerator2`
          (if (> (`KismetMathLibrary.Vector_Distance` (`KismetMathLibrary.MakeVector` (.x _returnvalue_6) (.y _returnvalue_6)) (`KismetMathLibrary.MakeVector` (.x _returnvalue_2) (.y _returnvalue_2))) (`self.DistanceTolerance`))
            (set `local.LocalRotation` (`KismetMathLibrary.MakeRotator` 180.0 0.0 (`KismetMathLibrary.DegAtan2` (* (.z (`KismetMathLibrary.Normal` (- _returnvalue_6 _returnvalue_2))) -1.0) (.x (`KismetMathLibrary.Normal` (- _returnvalue_6 _returnvalue_2))))))
            (else
              (return (struct) true))))
        (:`NewEnumerator3`
          (if (> (`KismetMathLibrary.Vector_Distance` (`KismetMathLibrary.MakeVector` (.x _returnvalue_5) 0.0 (.z _returnvalue_5)) (`KismetMathLibrary.MakeVector` (.x _returnvalue) 0.0 (.z _returnvalue))) (`self.DistanceTolerance`))
            (set `local.LocalRotation` (`KismetMathLibrary.MakeRotator` -90.0 (`KismetMathLibrary.DegAtan2` (* (.z (`KismetMathLibrary.Normal` (- _returnvalue_5 _returnvalue))) -1.0) (.x (`KismetMathLibrary.Normal` (- _returnvalue_5 _returnvalue))))))
            (else
              (return (struct) true)))))
      (return (`local.LocalRotation`) false))))

(fn `SetEndTile`
  (params (InInstigator :type "/Game/PortalSystem/DemoContent/ThirdPersonBP/Blueprints/BP_Deactivator3 Object Reference"))
  (locals (IgnoreActors :type "Array of Actor Object Reference"))
  (bind _returnvalue (`self.K2_GetActorLocation` (`local.InInstigator`)))
  (`KismetArrayLibrary.Array_Add` (`local.IgnoreActors`) InInstigator)
  (bind (_outhit _returnvalue_2) (`KismetSystemLibrary.LineTraceSingle` _returnvalue (+ _returnvalue (* (`self.GetActorUpVector` (`local.InInstigator`)) -100.0)) "TraceTypeQuery3" false (`local.IgnoreActors`)))
  (if _returnvalue_2
    (bind _asbp_tile (cast `/Game/Blueprints/Building/Tiles/BP_Tile` (`.HitActor` (`GameplayStatics.BreakHitResult` _outhit))))
    (bind _output_get (set `self.HitEndTile` _asbp_tile))
    (if (!= _output_get (`self.PrevHitEndTile`))
      (set `self.PrevHitEndTile` _output_get))))

(fn `SetPatrollingPath`
  (params (InNavGridGen :type "/Game/Blueprints/Building/BP_NavGridGenerator Object Reference"))
  (set `self.bPatrolling` true)
  (if (not (> (`self.NextPatrollingIndex`) 0))
    (bind _asbp_nav_grid (cast `/Game/Blueprints/Building/Grid/BP_NavGrid` (`self.GetOwner` (`self.HitStarTile`))))
    (bind _outrandomtile (`/Game/Blueprints/Building/Grid/BP_NavGrid.GetRandomWalkingTileTile` _asbp_nav_grid))
    (set `self.HitEndTile` _outrandomtile)
    (`/Game/Blueprints/Building/BP_NavGridGenerator.NavGridFindPathTo` (`local.InNavGridGen`) (`self.HitStarTile`) (`self.HitEndTile`) self)))

(fn `SetStartTile`
  (locals (IgnoreActors :type "Array of Actor Object Reference"))
  (bind _returnvalue (`self.K2_GetActorLocation`))
  (`KismetArrayLibrary.Array_Add` (`local.IgnoreActors`) self)
  (bind (_outhit _returnvalue_2) (`KismetSystemLibrary.LineTraceSingle` _returnvalue (+ _returnvalue (* (`self.GetActorUpVector`) -100.0)) "TraceTypeQuery3"))
  (if _returnvalue_2
    (bind _asbp_tile (cast `/Game/Blueprints/Building/Tiles/BP_Tile` (`.HitActor` (`GameplayStatics.BreakHitResult` _outhit))))
    (bind _output_get (set `self.HitStarTile` _asbp_tile))
    (if (!= _output_get (`self.PrevHitStarTile`))
      (set `self.PrevHitStarTile` _output_get))))

(fn `UserConstructionScript`)