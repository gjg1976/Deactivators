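; Player controller that lets the player pick a start and an end actor by mouse click to request a path between them.
; Enhanced Input clicks trace under the cursor for BPI_interactable actors and switch their color mode through interface messages.
; The first pick sets the start, the second sets the end and calls FindPathTo.
; Clicking the start again unselects it; clicking after a complete pair resets colors and calls DeselectPath.
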(event `self.ReceiveBeginPlay`
  (`self.SetupInput`))

(event `EnhancedInput|/Game/Blueprints/Inputs/Actions/AI_Click`
  (params (ActionValue :type Boolean) (ElapsedSeconds :type "Float (double-precision)") (TriggeredSeconds :type "Float (double-precision)") (InputAction :type "InputAction Object Reference" :default "/Game/Blueprints/Inputs/Actions/AI_Click.AI_Click"))
  (bind (_bfound _clickedactor) (`self.GetClickedActor`))
  (:`Triggered`
    (`|ExecutionSequence`
      (:`then_0`
        (`self.StartPath`
          (:`then`
            (`self.EndPath`
              (:`then`
                (message `/Game/Blueprints/Libraries/BPI_interactable.OnInteract` (`self.StartPath`) "NewEnumerator0")
                (message `/Game/Blueprints/Libraries/BPI_interactable.OnInteract` (`self.EndPath`) "NewEnumerator0")
                (`self.DeselectPath`))
              (:`else`)))
          (:`else`)))
      (:`then_1`
        (if _bfound
          (if (== _clickedactor (`self.StartPath`))
            (message `/Game/Blueprints/Libraries/BPI_interactable.OnInteract` (`self.StartPath`) "NewEnumerator0")
            (set `self.StartPath` null)
            (else
              (`self.StartPath`
                (:`then`
                  (`self.EndPath`
                    (:`then`
                      (bind _output_get (set `self.StartPath` _clickedactor :!label _label))
                      (message `/Game/Blueprints/Libraries/BPI_interactable.OnInteract` _output_get "NewEnumerator0" 0)
                      (set `self.EndPath` null))
                    (:`else`
                      (bind _output_get_2 (set `self.EndPath` _clickedactor))
                      (message `/Game/Blueprints/Libraries/BPI_interactable.OnInteract` _output_get_2 "NewEnumerator0" 0)
                      (`self.FindPathTo` (`self.StartPath`) (`self.EndPath`)))))
                (:`else`
                  (goto _label))))))))))

(event `EnhancedInput|/Game/Blueprints/Inputs/Actions/AI_Touch`
  (params (ActionValue :type Boolean) (ElapsedSeconds :type "Float (double-precision)") (TriggeredSeconds :type "Float (double-precision)") (InputAction :type "InputAction Object Reference" :default "/Game/Blueprints/Inputs/Actions/AI_Touch.AI_Touch")))

(fn `GetClickedActor`
  (returns (bFound :type Boolean) (ClickedActor :type "Actor Object Reference"))
  (bind (_bblockinghit _binitialoverlap _time _distance _location _impactpoint _normal _impactnormal _physmat _hitactor) (`GameplayStatics.BreakHitResult` (`self.GetHitResultUnderCursorByChannel` "TraceTypeQuery3")))
  (return (and _bblockinghit (`KismetSystemLibrary.DoesImplementInterface` _hitactor "/Game/Blueprints/Libraries/BPI_interactable.BPI_interactable_C")) _hitactor))

(fn `SetupInput`
  (bind _returnvalue (subsystem `EnhancedInputLocalPlayerSubsystem`))
  (`/Engine/EditorBlueprintResources/StandardMacros.IsValid` _returnvalue
    (:`Is Valid`
      (`EnhancedInputSubsystemInterface.AddMappingContext` _returnvalue "/Game/Blueprints/Inputs/IMC_Generator.IMC_Generator" 0 (struct)))))

(fn `UserConstructionScript`)